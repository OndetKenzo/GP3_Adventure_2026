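; Player combat component that runs a montage-based melee combo on the ground and a single attack in the air.
; Ground attacks step through AttackProfiles, optionally auto-face the closest enemy and launch forward, with montage notifies timing the combo window.
; Landing resets the combo and stops the air attack.
; TriggerHit sphere-traces between mesh sockets to apply damage, while the current mask's effects can block attacks or scale damage and ground attack speed.
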(event `self.ReceiveBeginPlay`
  (`parent.ReceiveBeginPlay`)
  (add `Character.LandedDelegate` (`self.player`) (`|CreateDelegate` :!event `OnCharacterLanded`)))

(event `TriggerAttack`
  (if (`self.CanAttackEffect`)
    (`self.canAttack`
      (:`then`
        (`/Game/Entities/Player/BP_Player.ActivateAttack` (`self.player`) "NewEnumerator1" "NewEnumerator0" "NewEnumerator0")
        (if (`NavMovementComponent.IsFalling` (`Character.CharacterMovement` (`self.player`)))
          (`self.AirAttack`)
          (else
            (`self.GroundAttack`))))
      (:`else`))))

(event `GroundAttack`
  (bind _attackindexcurrent (`self.attackIndexCurrent`))
  (bind _player (`self.player`))
  (`Actor.DisableInput` (`self.player`) (`GameplayStatics.GetPlayerController` 0))
  (`KismetArrayLibrary.Array_Clear` (`self.hitActors`))
  (bind _attackspeed (`self.AttackSpeedEffect`))
  ; Anim Notif (Combo Window)
  (`|ExecutionSequence`
    (:`then_0`
      (if (== (- (`KismetArrayLibrary.Array_Length` (`self.attackProfiles`)) 1) (`self.attackIndexCurrent`))
        (`self.OnCombot`)))
    (:`then_1`
      (bind _notifyname (`|PlayMontage` (`self.mesh`) (`/Game/Entities/Player/PDA_PlayerAttacks.animation` (`|GetArrayItem` (`self.attackProfiles`) (`self.attackIndexCurrent`))) _attackspeed)
        (:`then`
          (`|ExecutionSequence`
            (:`then_0`
              (if (`self.hasAutoTarget`)
                ; Auto-Target System (Player turns to closest Enemy)
                (bind (_enemy _impactpoint _hascloseenemy) (`self.FindClosestEnemy` (`self.autoTargetRange`)))
                (if _hascloseenemy
                  (bind (_returnvalue_roll _returnvalue_pitch _returnvalue_yaw) (`KismetMathLibrary.BreakRotator` (`KismetMathLibrary.FindLookAtRotation` (`Actor.K2_GetActorLocation` _player) (`Actor.K2_GetActorLocation` _enemy))))
                  (`Actor.K2_SetActorRotation` _player (`KismetMathLibrary.MakeRotator` 0.0 0.0 _returnvalue_yaw) false))))
            (:`then_1`
              (`/Game/Entities/Player/BP_Player.ForwardLaunch` (`self.player`) (`/Game/Entities/Player/PDA_PlayerAttacks.forwardLaunch` (`|GetArrayItem` (`self.attackProfiles`) (`self.attackIndexCurrent`)))))
            (:`then_2`
              ; Uses Next Combo Attack Anim
              (set `self.attackIndexCurrent` (`KismetMathLibrary.SelectInt` (+ _attackindexcurrent 1) 0 (< _attackindexcurrent (`KismetArrayLibrary.Array_LastIndex` (`self.attackProfiles`))))))))
        (:`OnCompleted`
          (`/Game/Entities/Player/BP_Player.ActivateAttack` (`self.player`) "NewEnumerator0" "NewEnumerator0" "NewEnumerator0")
          (set `self.attackIndexCurrent` 0)
          (`Actor.EnableInput` (`self.player`) (`GameplayStatics.GetPlayerController` 0)))
        (:`OnInterrupted`
          ;; FIX Soft lock after falling attack
          (`Actor.EnableInput` (`self.player`) (`GameplayStatics.GetPlayerController` 0))
          (`KismetSystemLibrary.Delay` 0.5)
          (`/Game/Entities/Player/BP_Player.ActivateAttack` (`self.player`) "NewEnumerator0" "NewEnumerator2" "NewEnumerator2"))
        (:`OnNotifyBegin`
          (switch `name` _notifyname
            (:`ComboInputWindow`
              (`/Game/Entities/Player/BP_Player.ActivateAttack` (`self.player`) "NewEnumerator0" "NewEnumerator2" "NewEnumerator2")
              (`Actor.EnableInput` (`self.player`) (`GameplayStatics.GetPlayerController` 0)))))
        (:`OnNotifyEnd`
          (switch `name` _notifyname
            (:`ComboInputWindow`
              (`/Game/Entities/Player/BP_Player.ActivateAttack` (`self.player`) "NewEnumerator1" "NewEnumerator2" "NewEnumerator2")
              (`Actor.DisableInput` (`self.player`) (`GameplayStatics.GetPlayerController` 0)))))))))

(event `AirAttack`
  (`KismetArrayLibrary.Array_Clear` (`self.hitActors`))
  (`|PlayMontage` (`self.mesh`) (`/Game/Entities/Player/PDA_PlayerAttacks.animation` (`self.airAttackProfile`))
    (:`OnCompleted`
      _)
    (:`OnBlendOut`
      _)
    (:`OnInterrupted`
      _))
  (`/Game/Entities/Player/BP_Player.ActivateAttack` (`self.player`) "NewEnumerator0" "NewEnumerator0" "NewEnumerator0")
  (`Actor.EnableInput` (`self.player`) (`GameplayStatics.GetPlayerController` 0)))

(event `OnCharacterLanded`
  (params (Hit :type "HitResult Structure (by ref)"))
  (set `self.attackIndexCurrent` 0)
  (if (== (`Character.GetCurrentMontage` (`self.player`)) (`/Game/Entities/Player/PDA_PlayerAttacks.animation` (`self.airAttackProfile`)))
    (`Character.StopAnimMontage` (`self.player`) (`/Game/Entities/Player/PDA_PlayerAttacks.animation` (`self.airAttackProfile`)))
    (`/Game/Entities/Player/BP_Player.ActivateAttack` (`self.player`) "NewEnumerator0" "NewEnumerator0" "NewEnumerator0")))

(event `TriggerHit`
  (params (AttackType :type "/Game/Entities/Player/PDA_PlayerAttacks Object Reference"))
  (bind _mesh (`self.mesh`))
  (bind (_outhits _returnvalue) (`KismetSystemLibrary.SphereTraceMultiForObjects` (`SceneComponent.GetSocketLocation` _mesh (`/Game/Entities/Player/PDA_PlayerAttacks.startSocket` AttackType)) (`SceneComponent.GetSocketLocation` _mesh (`/Game/Entities/Player/PDA_PlayerAttacks.endSocket` AttackType)) (* (`/Game/Entities/Player/PDA_PlayerAttacks.hitSphereRadius` AttackType) 15.0) (`/Game/Entities/Player/PDA_PlayerAttacks.hitableObjectTypes` AttackType)))
  (`self.ApplyDamageToHitActors` AttackType _returnvalue _outhits (`self.AttackDamageEffect`)))

(fn `AttackDamageEffect`
  (returns (DamageMultiplier :type "Float (double-precision)"))
  (bind (_value _returnvalue) (`BlueprintMapLibrary.Map_Find` (`/Game/Entities/Player/PDA_MaskProfile.maskEffect` (`/Game/Entities/Player/AC_MaskSystem.currentMask` (`self.maskSystemComponent`))) "NewEnumerator4"))
  (if _returnvalue
    (return _value)
    (else
      (return 1.0))))

(fn `AttackSpeedEffect`
  (returns (AttackSpeed :type "Float (double-precision)"))
  (bind (_value _returnvalue) (`BlueprintMapLibrary.Map_Find` (`/Game/Entities/Player/PDA_MaskProfile.maskEffect` (`/Game/Entities/Player/AC_MaskSystem.currentMask` (`self.maskSystemComponent`))) "NewEnumerator1"))
  (if _returnvalue
    (return _value)
    (else
      (return 1.0))))

(fn `CanAttackEffect`
  (returns (canAttack :type Boolean))
  (return (not (`.ReturnValue` (`BlueprintMapLibrary.Map_Find` (`/Game/Entities/Player/PDA_MaskProfile.maskEffect` (`/Game/Entities/Player/AC_MaskSystem.currentMask` (`self.maskSystemComponent`))) "NewEnumerator7")))))