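; Player combat component that runs the parry action and its impact feedback.
; Parry toggles the player's attack, parry and shoot permissions, sets IsParrying and plays a whoosh and montage.
; When the montage completes, it clears the flag, toggles those permissions again and enables input.
; ActionJuice plays parry sound, counter and shockwave Niagara effects in front of the player, camera shake and brief global slow motion.
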(event `Parry`
  (`self.canParry`
    (:`then`
      (`/Game/Entities/Player/BP_Player.ActivateAttack` (`self.player`) "NewEnumerator1" "NewEnumerator1" "NewEnumerator1")
      (set `self.isParrying` true)
      (`GameplayStatics.PlaySoundAtLocation` "/Game/Placeholder/SFX/SC_Woosh.SC_Woosh" (`Actor.K2_GetActorLocation` (`self.player`)) (struct) 1.0 1.0 0.0 null null null null)
      (`|PlayMontage` (`self.mesh`) (`self.parryAnim`)
        (:`OnCompleted`
          (set `self.isParrying` false)
          (`/Game/Entities/Player/BP_Player.ActivateAttack` (`self.player`) "NewEnumerator0" "NewEnumerator0" "NewEnumerator0")
          (`Actor.EnableInput` (`self.player`) (`GameplayStatics.GetPlayerController` 0)))))
    (:`else`)))

(event `SlowTime`
  (`GameplayStatics.SetGlobalTimeDilation` 0.5)
  (`KismetSystemLibrary.Delay` 0.5)
  (`GameplayStatics.SetGlobalTimeDilation` 1.0))

(fn `ActionJuice`
  (params (HitInfo :type "HitResult Structure (by ref)") (HitActor :type "Actor Object Reference") (IsHitActorDying :type Boolean))
  (bind _player (`self.player`))
  (bind _returnvalue (`Actor.K2_GetActorLocation` _player))
  (bind _returnvalue_2 (+ _returnvalue (* (`SceneComponent.GetForwardVector` (`Actor.RootComponent` _player)) 80)))
  (`GameplayStatics.PlaySoundAtLocation` "/Game/Placeholder/SFX/SC_Parry.SC_Parry" _returnvalue (struct) 1.0 1.0 0.0 null null null null)
  (`NiagaraFunctionLibrary.SpawnSystemAtLocation` "/Game/FX/Protagonist/Counter/NS_Prota_Perfect_Counter.NS_Prota_Perfect_Counter" _returnvalue_2)
  (`NiagaraFunctionLibrary.SpawnSystemAtLocation` "/Game/Entities/Player/VFX/NS_Shockwave.NS_Shockwave" _returnvalue_2)
  (`PlayerCameraManager.StartCameraShake` :`self` (`PlayerController.PlayerCameraManager` (`GameplayStatics.GetPlayerController` 0)) :`ShakeClass` "/Game/Entities/Player/VFX/CSB_CamParry.CSB_CamParry_C")
  (`self.SlowTime`)
  (return))