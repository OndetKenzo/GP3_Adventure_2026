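; Player gun component that runs a cooldown-limited shot at the closest enemy in range, or into the air if none is found.
; Shooting spawns a socketed gun, changes action permissions and flags the Anim Blueprint or plays a fire-up montage.
; Separate juice events handle effects, sound and enemy damage, while a looping timer drives an overhead cooldown bar.
; The current mask can add healing, scale cooldown speed or chain repeat shots that bypass the cooldown.
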(event `self.ReceiveBeginPlay`
  (`parent.ReceiveBeginPlay`)
  (`self.SpawnTimerBar`))

(event `Shoot`
  (bind _timerbar (`self.timerBar`))
  (`self.canShoot`
    (:`then`
      (if (<= (`self.gunCooldownTimer`) 0.0)
        (set `self.gunCooldownTimer` (`self.gunCooldownDuration`))
        (`/Game/Entities/Player/BP_Player.ActivateAttack` (`self.player`) "NewEnumerator1" "NewEnumerator1" "NewEnumerator1" :!label _label)
        ; Attach Gun
        (bind _returnvalue (`|SpawnActorFromClass` "/Game/Entities/Player/Animation/BP_Gun.BP_Gun_C" (`SceneComponent.GetSocketTransform` (`self.mesh`) "gun" "RTS_World") "Undefined" "MultiplyWithRoot" null null))
        (set `self.currentGun` _returnvalue)
        (`Actor.K2_AttachToComponent` _returnvalue (`self.mesh`) "gun" "SnapToTarget" "SnapToTarget" "SnapToTarget" true)
        ; GunTimer
        (`Widget.SetVisibility` _timerbar "Visible")
        (`/Game/Entities/Player/VFX/WBP_GunTimer.SetFillLevel` _timerbar 1.0)
        (`KismetSystemLibrary.K2_SetTimerDelegate` (`|CreateDelegate` :!event `GunTimerUpdate`) (`GameplayStatics.GetWorldDeltaSeconds`) true)
        ; Check If there are Ennemies Close by
        (bind (_enemy _impactpoint _hascloseenemy) (`self.FindClosestEnemy` (`self.shootRange`)))
        (`KismetSystemLibrary.PrintString` (`KismetStringLibrary.Conv_BoolToString` _hascloseenemy) true true (struct :`R` 1.0 :`G` 0.008477 :`A` 1.0))
        (`KismetSystemLibrary.PrintString` (`KismetSystemLibrary.GetDisplayName` _enemy))
        (set `self.enemyTarget` _enemy)
        (if _hascloseenemy
          ;; This plays the Shoot Animation in ABP
          (set `self.isShootingEnemy` true)
          (`KismetSystemLibrary.K2_SetTimerDelegate` (`|CreateDelegate` :!event `EndShooting`) (`AnimSequenceBase.SequenceLength` (`self.animShoot`)))
          (else
            (`self.OnFireUp`)
            (`|PlayMontage` (`self.mesh`) (`self.animShootUp`)
              (:`OnCompleted`
                (`self.EndShooting`)))))))
    (:`else`)))

(event `MultiShotStart`
  (goto _label))

(event `EndShooting`
  (bind (_value _returnvalue) (`BlueprintMapLibrary.Map_Find` (`/Game/Entities/Player/PDA_MaskProfile.maskEffect` (`/Game/Entities/Player/AC_MaskSystem.currentMask` (`self.maskSystemComponent`))) "NewEnumerator5"))
  (`Actor.K2_DestroyActor` (`self.currentGun`))
  (set `self.isShootingEnemy` false)
  (set `self.enemyTarget` null)
  (`/Game/Entities/Player/BP_Player.ActivateAttack` (`self.player`) "NewEnumerator0" "NewEnumerator0" "NewEnumerator0")
  (`Actor.EnableInput` (`self.player`) (`GameplayStatics.GetPlayerController` 0))
  (if _returnvalue
    (`self.MultiGunShotEffect` (`KismetMathLibrary.FTrunc` _value))))

(event `SpawnTimerBar`
  (bind _player (`self.player`))
  (bind _timerbar (`self.timerBar`))
  (bind _returnvalue (`|CreateWidget` "/Game/Entities/Player/VFX/WBP_GunTimer.WBP_GunTimer_C"))
  (set `self.timerBar` _returnvalue)
  (bind _returnvalue_2 (`|AddComponentByClass` _player "/Script/UMG.WidgetComponent" false (`KismetMathLibrary.MakeTransform` (`KismetMathLibrary.MakeVector` 0.0 0.0 (+ (`CapsuleComponent.CapsuleHalfHeight` (`Character.CapsuleComponent` _player)) (`self.healthBarZ_Offset`))))))
  (`WidgetComponent.SetWidgetSpace` _returnvalue_2 "Screen")
  (`WidgetComponent.SetWidget` _returnvalue_2 _timerbar)
  (`WidgetComponent.SetDrawSize` _returnvalue_2 (`self.healthBarSize`))
  (`Widget.SetVisibility` _timerbar "Hidden"))

(event `MultiGunShotEffect`
  (params (`Number of Shots` :type Integer))
  (bind _output_get (set `self.gunShootNumber` (+ (`self.gunShootNumber`) 1)))
  (`KismetSystemLibrary.PrintString` (`KismetStringLibrary.Conv_IntToString` _output_get))
  (if (>= _output_get `Number of Shots`)
    (set `self.gunShootNumber` 0)
    (else
      (`KismetSystemLibrary.PrintString` "Hello")
      (`KismetSystemLibrary.Delay` (`self.betweenShotsTimer`))
      (`self.MultiShotStart`))))

(event `GunTimerUpdate`
  (bind _output_get (set `self.gunCooldownTimer` (- (`self.gunCooldownTimer`) (`self.GunCooldownEffect` (`GameplayStatics.GetWorldDeltaSeconds`)))))
  (`/Game/Entities/Player/VFX/WBP_GunTimer.SetFillLevel` (`self.timerBar`) (/ _output_get (`self.gunCooldownDuration`)))
  (if (<= (`self.gunCooldownTimer`) 0.0)
    (`Widget.SetVisibility` (`self.timerBar`) "Hidden")))

(event `ShootUpJuice`
  (`NiagaraFunctionLibrary.SpawnSystemAtLocation` "/Game/Placeholder/Vefects/Easy_Shockwaves_VFX/VFX/Shockwaves/Particles/Color_Variation/VFX_Shockwave_01_Black_Big_1s.VFX_Shockwave_01_Black_Big_1s" (- (`Actor.K2_GetActorLocation` (`self.player`)) (0.0 0.0 80.0)))
  (`GameplayStatics.PlaySound2D` "/Game/Placeholder/SFX/Gun_Shoot_Up.Gun_Shoot_Up" 1.0 1.0 0.0 null null))

(event `ShootEnemyJuice`
  (bind _returnvalue (`Actor.GetComponentByClass` (`self.player`) "AC_GunSystem_C"))
  (bind _enemytarget (`/Game/Entities/Player/PlayerCombatSystem/AC_GunSystem.enemyTarget` _returnvalue))
  (bind _returnvalue_2 (`Actor.K2_GetActorLocation` _enemytarget))
  (`self.ApplyDamageToActor` _returnvalue _enemytarget (`/Game/Entities/Player/PlayerCombatSystem/AC_GunSystem.shootDamage` _returnvalue) (`GameplayStatics.MakeHitResult` false false 0.0 0.0 _returnvalue_2 _returnvalue_2 (0.0 0.0 1.0) (0.0 0.0 1.0) null _enemytarget) 0.0)
  (`GameplayStatics.PlaySound2D` "/Game/Placeholder/SFX/Gun_Shoot.Gun_Shoot" 1.0 1.0 0.0 null null)
  (`self.GunHealEffect`))

(fn `ActionJuice`
  (params (HitInfo :type "HitResult Structure (by ref)") (HitActor :type "Actor Object Reference") (IsHitActorDying :type Boolean))
  (`parent.ActionJuice` HitInfo HitActor false)
  (return))

(fn `GunCooldownEffect`
  (params (cooldownInput :type "Float (double-precision)"))
  (returns (cooldownOutput :type "Float (double-precision)"))
  (bind (_value _returnvalue) (`BlueprintMapLibrary.Map_Find` (`/Game/Entities/Player/PDA_MaskProfile.maskEffect` (`/Game/Entities/Player/AC_MaskSystem.currentMask` (`self.maskSystemComponent`))) "NewEnumerator6"))
  (if _returnvalue
    (return (* _value cooldownInput))
    (else
      (return cooldownInput))))

(fn `GunHealEffect`
  (bind (_value _returnvalue) (`BlueprintMapLibrary.Map_Find` (`/Game/Entities/Player/PDA_MaskProfile.maskEffect` (`/Game/Entities/Player/AC_MaskSystem.currentMask` (`self.maskSystemComponent`))) "NewEnumerator0"))
  (if _returnvalue
    (`/Game/Entities/Player/AC_PlayerHealthSystem.Heal` (`self.healthSystem`) (`KismetMathLibrary.FTrunc` _value))))