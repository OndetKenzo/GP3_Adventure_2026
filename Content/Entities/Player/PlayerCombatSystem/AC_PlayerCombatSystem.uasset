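; Player combat component that applies melee hit damage to enemies and plays the hit feedback.
; BeginPlay caches player components, enables custom depth on the mesh and ensures a hit-stop component exists.
; Each character not already in HitActors takes multiplied point damage, optional stagger and, if still alive, knockback.
; Survivors trigger camera shake and hit stop, killing blows play a finisher sound, and a sphere-trace helper finds nearby enemies.
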(event `self.ReceiveBeginPlay`
  (bind _returnvalue (`self.GetOwner`))
  (bind _player (`self.player`))
  (bind _mesh (`self.mesh`))
  (bind _returnvalue_2 (`Actor.GetComponentByClass` (`self.player`) "/Game/Entities/Player/AC_HitStop.AC_HitStop_C"))
  ; SetupVariable
  (if (`KismetSystemLibrary.DoesImplementInterface` _returnvalue "/Game/Entities/Player/BPI_IsPlayer.BPI_IsPlayer_C")
    (bind _bp_player (message `/Game/Entities/Player/BPI_IsPlayer.IsPlayer` _returnvalue))
    (bind _output_get (set `self.player` _bp_player))
    (set `self.mesh` (`Character.Mesh` _output_get))
    (set `self.maskSystemComponent` (`Actor.GetComponentByClass` _player "/Game/Entities/Player/AC_MaskSystem.AC_MaskSystem_C"))
    (set `self.healthSystem` (`Actor.GetComponentByClass` _player "/Game/Entities/Player/AC_PlayerHealthSystem.AC_PlayerHealthSystem_C"))
    ; Juice Setup
    (`PrimitiveComponent.SetRenderCustomDepth` _mesh true)
    (`PrimitiveComponent.SetCustomDepthStencilValue` _mesh 1)
    (`/Engine/EditorBlueprintResources/StandardMacros.IsValid` _returnvalue_2
      (:`Is Valid`
        (set `self.hitStopComp` _returnvalue_2))
      (:`Is Not Valid`
        (bind _returnvalue_3 (`|AddComponentByClass` (`self.player`) "/Game/Entities/Player/AC_HitStop.AC_HitStop_C"))
        (set `self.hitStopComp` _returnvalue_3)))))

(fn `ActionJuice`
  (params (HitInfo :type "HitResult Structure (by ref)") (HitActor :type "Actor Object Reference") (IsHitActorDying :type Boolean))
  (bind _returnvalue (`Actor.K2_GetActorLocation` HitActor))
  (bind _returnvalue_2 (`Actor.GetComponentByClass` (`local.HitActor`) "/Game/Entities/Player/AC_HitStop.AC_HitStop_C"))
  (if IsHitActorDying
    (`GameplayStatics.PlaySoundAtLocation` "/Game/Placeholder/SFX/Punch_Finisher.Punch_Finisher" _returnvalue (struct) 1.0 1.0 0.0 null null null null)
    (else
      (`GameplayStatics.PlaySoundAtLocation` "/Game/Placeholder/SFX/SC_Punch.SC_Punch" _returnvalue (struct) 1.0 1.0 0.0 null null null null)
      (`PlayerCameraManager.StartCameraShake` :`self` (`PlayerController.PlayerCameraManager` (`GameplayStatics.GetPlayerController` 0)) :`ShakeClass` "/Game/Entities/Player/VFX/CSB_CamHitShake.CSB_CamHitShake_C")
      (`/Game/Entities/Player/AC_HitStop.BeginHitStop` (`self.hitStopComp`) 0.15 0.05 30.0 1.0 false)
      (`/Engine/EditorBlueprintResources/StandardMacros.IsValid` _returnvalue_2
        (:`Is Valid`
          (`/Game/Entities/Player/AC_HitStop.BeginHitStop` _returnvalue_2 0.15 0.0 30.0 20.0 true))))))

(fn `ApplyDamageToActor`
  (params (EnemyTarget :type "Character Object Reference") (AttackType :type "/Game/Entities/Player/PDA_PlayerAttacks Object Reference") (HitInfo :type "HitResult Structure (by ref)") (DamageMultiplier :type "Float (double-precision)"))
  (locals (HitActor :type "Actor Object Reference") (HitResult :type "HitResult Structure"))
  (bind _isdying (`self.CheckIfHitActorIsDying` EnemyTarget))
  (bind _attacktype (`local.AttackType`))
  (bind _enemytarget (`local.EnemyTarget`))
  (bind _attacktype_2 (`local.AttackType`))
  (`GameplayStatics.ApplyPointDamage` EnemyTarget (* (`KismetMathLibrary.Conv_IntToDouble` (`/Game/Entities/Player/PDA_PlayerAttacks.damage` AttackType)) DamageMultiplier) (0.0 0.0 0.0) HitInfo null (`self.player`))
  (`self.ActionJuice` (`local.HitInfo`) (`local.EnemyTarget`) _isdying)
  (`|ExecutionSequence`
    (:`then_0`
      (if (`/Game/Entities/Player/PDA_PlayerAttacks.doStagger` _attacktype_2)
        (message `/Game/Entities/Player/BPI_IsEnemy.SetStunState` (`local.EnemyTarget`) (`/Game/Entities/Player/PDA_PlayerAttacks.staggerTimer` _attacktype_2))))
    (:`then_1`
      (if _isdying
        _
        (elif (`/Game/Entities/Player/PDA_PlayerAttacks.doKnockback` _attacktype)
          (`Character.LaunchCharacter` _enemytarget (* (`KismetMathLibrary.Normal` (- (`Actor.K2_GetActorLocation` _enemytarget) (`Actor.K2_GetActorLocation` (`self.player`)))) (`/Game/Entities/Player/PDA_PlayerAttacks.knockbackDistance` _attacktype)) false false))))))

(fn `ApplyDamageToHitActors`
  (params (AttackType :type "/Game/Entities/Player/PDA_PlayerAttacks Object Reference") (Hit :type Boolean) (Hits :type "Array of HitResult Structure") (DamageMutiplier :type "Float (double-precision)"))
  (locals (HitActor :type "Character Object Reference") (HitResult :type "HitResult Structure"))
  (if Hit
    (`AkGameplayStatics.PostEvent` "/Game/WwiseAudio/Events/Default_Work_Unit/ENNEMIES/Play_SFX_ENEMYHIT.Play_SFX_ENEMYHIT")
    (for _array_element Hits
      (set `local.HitResult` _array_element)
      (bind _ascharacter (cast `Character` (`.HitActor` (`GameplayStatics.BreakHitResult` _array_element))))
      (set `local.HitActor` _ascharacter)
      (if (not (`KismetArrayLibrary.Array_Contains` (`self.hitActors`) (`local.HitActor`)))
        (`self.ApplyDamageToActor` (`local.HitActor`) (`local.AttackType`) (`local.HitResult`) (`local.DamageMutiplier`))
        (`KismetArrayLibrary.Array_Add` (`self.hitActors`) (`local.HitActor`))))))

(fn `CheckIfHitActorIsDying`
  (params (HitActor :type "Actor Object Reference"))
  (returns (IsDying :type Boolean))
  (if (`KismetSystemLibrary.DoesImplementInterface` HitActor "/Game/Entities/Player/BPI_IsEnemy.BPI_IsEnemy_C")
    (bind _bp_enemy (message `/Game/Entities/Player/BPI_IsEnemy.IsEnemy` HitActor))
    (return (<= (`/Game/Entities/Player/AC_EnemyHealthSystem.currentHeathPoints` (`Actor.GetComponentByClass` _bp_enemy "/Game/Entities/Player/AC_EnemyHealthSystem.AC_EnemyHealthSystem_C")) 0.0))))

(fn `FindClosestEnemy`
  (params (Range :type "Float (single-precision)"))
  (returns (Enemy :type "/Game/Entities/NPCs/Enemies/BP/BP_MasterEnemy Object Reference") (ImpactPoint :type "Vector Structure") (HasCloseEnemy :type Boolean))
  (bind _returnvalue (`Actor.K2_GetActorLocation` (`self.GetOwner`)))
  (bind (_outhit _returnvalue_2) (`KismetSystemLibrary.SphereTraceSingleForObjects` _returnvalue _returnvalue Range (`|MakeArray` "ObjectTypeQuery3" :!type "EObjectTypeQuery Enum") false (`|MakeArray` null :!type "Actor Object Reference")))
  (if _returnvalue_2
    (bind (_bblockinghit _binitialoverlap _time _distance _location _impactpoint _normal _impactnormal _physmat _hitactor) (`GameplayStatics.BreakHitResult` _outhit))
    (if (`KismetSystemLibrary.DoesImplementInterface` _hitactor "/Game/Entities/Player/BPI_IsEnemy.BPI_IsEnemy_C")
      (bind _bp_enemy (message `/Game/Entities/Player/BPI_IsEnemy.IsEnemy` _hitactor))
      (return _bp_enemy _impactpoint true)
      (else
        _)))
  (return null (0.0 0.0 0.0) false))