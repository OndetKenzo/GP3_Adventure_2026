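; Actor component that gives a Character a hit stop: time dilation, mesh shake and an optional flash overlay.
; BeginHitStop sets CustomTimeDilation, starts shake and duration timers, and can apply a dynamic M_HitFlash overlay.
; Shake steps offset the mesh along the camera's right vector in actor-local XY, scaled by amplitude, OffsetDirection and a ShakeResolve curve over elapsed time.
; EndHitStop restores time dilation, mesh position and overlay.
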(event `self.ReceiveBeginPlay`
  (bind _ascharacter (cast `Character` (`self.GetOwner`)))
  (bind _output_get (set `self.CharacterActor` _ascharacter))
  (bind _mesh (`Character.Mesh` _output_get))
  (set `self.Mesh` _mesh)
  (set `self.MeshDefaultRelativeLoc` (`SceneComponent.RelativeLocation` _mesh))
  (bind _returnvalue (`KismetMaterialLibrary.CreateDynamicMaterialInstance` "/Game/Entities/Player/VFX/M_HitFlash.M_HitFlash"))
  (bind _output_get_2 (set `self.HitFlashMaterial` _returnvalue))
  (`MaterialInstanceDynamic.SetScalarParameterValue` _output_get_2 "Speed" 20.0))

(event `BeginHitStop`
  (params (Duration :type "Float (double-precision)") (TimeDilation :type "Float (double-precision)") (ShakeSpeed :type "Float (double-precision)") (ShakeAmplitude :type "Float (double-precision)") (Flash :type Boolean))
  (set `self.Flash` Flash)
  (set `self.ShakeAmplitude` ShakeAmplitude)
  (bind _returnvalue (`KismetSystemLibrary.K2_SetTimerDelegate` (`|CreateDelegate` :!event `ApplyMeshShakeStep`) (/ 1.0 ShakeSpeed) true))
  (set `self.ShakeTimer` _returnvalue)
  (set `Actor.CustomTimeDilation` TimeDilation (`self.CharacterActor`))
  (bind _returnvalue_2 (`KismetSystemLibrary.K2_SetTimerDelegate` (`|CreateDelegate` :!event `EndHitStop`) Duration))
  (set `self.HitStopTimer` _returnvalue_2)
  (set `self.HitStopDuration` Duration)
  (`self.Flash`
    (:`then`
      (`MeshComponent.SetOverlayMaterial` (`self.Mesh`) (`self.HitFlashMaterial`)))
    (:`else`)))

(event `EndHitStop`
  (`KismetSystemLibrary.K2_ClearAndInvalidateTimerHandle` (`self.ShakeTimer`))
  (`SceneComponent.K2_SetRelativeLocation` (`self.Mesh`) (`self.MeshDefaultRelativeLoc`) false true)
  (set `Actor.CustomTimeDilation` 1.0 (`self.CharacterActor`))
  (`self.Flash`
    (:`then`
      (`MeshComponent.SetOverlayMaterial` (`self.Mesh`) null))
    (:`else`)))

(event `ApplyMeshShakeStep`
  (bind (_returnvalue_x _returnvalue_y) (`KismetMathLibrary.BreakVector` (`KismetMathLibrary.InverseTransformDirection` (`Actor.GetTransform` (`self.CharacterActor`)) (`Actor.GetActorRightVector` (`PlayerController.PlayerCameraManager` (`GameplayStatics.GetPlayerController` 0))))))
  (`SceneComponent.K2_SetRelativeLocation` (`self.Mesh`) (+ (`self.MeshDefaultRelativeLoc`) (* (`KismetMathLibrary.MakeVector` _returnvalue_x _returnvalue_y) (* (`self.ShakeAmplitude`) (`self.OffsetDirection`)) (`CurveFloat.GetFloatValue` (`self.ShakeResolve`) (/ (`KismetSystemLibrary.K2_GetTimerElapsedTimeHandle` (`self.HitStopTimer`)) (`self.HitStopDuration`))))) false true)
  (`/Engine/EditorBlueprintResources/StandardMacros.NegateFloat` (`self.OffsetDirection`)))