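; Enemy health component for Characters that turns point damage into directional hit-react montages, impact VFX and health bar updates.
; Damage passes through an activate/deactivate gate, and OnFirstHit handles health bar creation, static camera and Elite combat state.
; Death ragdolls the enemy away from the damage causer; ground contact or a fallback timer then swaps in a field-driven shatter asset and triggers any mask drop.
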(event `self.ReceiveBeginPlay`
  (bind _returnvalue (`Actor.GetComponentByClass` (`self.characterActor`) "/Game/Entities/Player/AC_HitStop.AC_HitStop_C"))
  (bind _ascharacter (cast `Character` (`self.GetOwner`)))
  (bind _output_get (set `self.characterActor` _ascharacter))
  (set `self.mesh` (`Character.Mesh` _ascharacter))
  (add `Actor.OnTakePointDamage` _output_get (`|CreateDelegate` :!event `OnTakePointDamage_Event`))
  (set `self.currentHeathPoints` (`self.maxHeathPoints`))
  (`/Engine/EditorBlueprintResources/StandardMacros.IsValid` _returnvalue
    (:`Is Valid`
      (set `self.hitStopComp` _returnvalue))
    (:`Is Not Valid`
      (bind _returnvalue_2 (`|AddComponentByClass` (`self.characterActor`) "/Game/Entities/Player/AC_HitStop.AC_HitStop_C"))
      (set `self.hitStopComp` _returnvalue_2))))

(event `Death`
  (params (DamageCauser :type "Actor Object Reference"))
  (bind _mesh (`self.mesh`))
  (bind _characteractor (`self.characterActor`))
  (bind _characteractor_2 (`self.characterActor`))
  (bind _returnvalue (`Actor.K2_GetActorLocation` (`self.characterActor`)))
  (bind _returnvalue_2 (`Actor.GetComponentByClass` (`self.characterActor`) "/Game/Entities/Player/AC_HitStop.AC_HitStop_C"))
  (bind _mesh_2 (`Character.Mesh` _characteractor_2))
  (bind _returnvalue_3 (`KismetMathLibrary.Normal` (- _returnvalue (`Actor.K2_GetActorLocation` DamageCauser))))
  (bind (_returnvalue_x _returnvalue_y) (`KismetMathLibrary.BreakVector` (* _returnvalue_3 (`self.dieImpulse`))))
  (`self.DoDeath`
    (:`then`
      (`AkGameplayStatics.PostEvent` "/Game/WwiseAudio/Events/Default_Work_Unit/ENNEMIES/Play_SFX_ENEMY_KILLED.Play_SFX_ENEMY_KILLED")
      (`AkGameplayStatics.PostEvent` "/Game/WwiseAudio/Events/Default_Work_Unit/VOICES/Play_Barks_Laughs.Play_Barks_Laughs")
      (`self.ReturnToMainCamera`)
      ; Setup
      (bind _healthbar (`self.healthBar`)
        (:`then`
          (`Widget.SetVisibility` _healthbar "Hidden"))
        (:`else`
          _))
      (`Character.StopAnimMontage` _characteractor_2 null)
      (set `Actor.bCanBeDamaged` false _characteractor_2)
      (`PrimitiveComponent.SetCollisionEnabled` _mesh_2 "QueryAndPhysics")
      (`|ExecutionSequence`
        (:`then_0`
          (`/Engine/EditorBlueprintResources/StandardMacros.IsValid` _returnvalue_2
            (:`Is Valid`
              (`self.K2_DestroyComponent` _returnvalue_2)
              (`self.OnDeath`)
              (bind _asgm_base (cast `/Game/Core/GameModes/Game/GM_Base` (`GameplayStatics.GetGameMode`)))
              (set `/Game/Core/GameModes/Game/GM_Base.isInCombat` false _asgm_base))))
        (:`then_1`
          ; Ragdoll
          (`PrimitiveComponent.SetSimulatePhysics` _mesh_2 true)
          (`PrimitiveComponent.SetCollisionResponseToChannel` (`Character.CapsuleComponent` _characteractor) "ECC_Pawn" "ECR_Ignore")
          (`Actor.K2_SetActorLocation` _characteractor (+ _returnvalue (0.0 0.0 100.0)) false true)
          (`KismetSystemLibrary.Delay` 0.05)
          (set `self.HitDirection` _returnvalue_3)
          (`PrimitiveComponent.AddImpulse` (`self.mesh`) (`KismetMathLibrary.MakeVector` _returnvalue_x _returnvalue_y (`self.dieImpulseUp`)) "None" true)
          (`PrimitiveComponent.SetNotifyRigidBodyCollision` _mesh true)
          (`PrimitiveComponent.SetCollisionResponseToChannel` _mesh "ECC_WorldStatic" "ECR_Block")
          (add `PrimitiveComponent.OnComponentHit` _mesh (`|CreateDelegate` :!event `OnGroundHit`))
          ; Temp Fix
          (`KismetSystemLibrary.K2_SetTimerDelegate` (`|CreateDelegate` :!event `StartDeath`) (`self.timeBeforeDeath`)))))
    (:`else`)))

(event `ActivateDamage`
  (goto _label :!via `Open`))

(event `DeactivateDamage`
  (goto _label :!via `Close`))

(event `OnTakePointDamage_Event`
  (params (DamagedActor :type "Actor Object Reference") (Damage :type "Float (single-precision)") (InstigatedBy :type "Controller Object Reference") (HitLocation :type "Vector Structure") (FHitComponent :type "PrimitiveComponent Object Reference") (BoneName :type Name) (ShotFromDirection :type "Vector Structure") (DamageType :type "DamageType Object Reference") (DamageCauser :type "Actor Object Reference"))
  ; Take Damage
  (`/Engine/EditorBlueprintResources/StandardMacros.Gate` false :!label _label
    (:`Exit`
      (`|PlayMontage` (`Character.Mesh` (`self.characterActor`)) (`BlueprintMapLibrary.Map_Find` (`self.hitReactAnimations`) (`self.HitLocationToDirection` HitLocation))
        (:`then`
          (`self.ProcessDamage` Damage DamageCauser)
          (`self.PlayerDamage`))))))

(event `ProcessDamage`
  (params (DamageAmount :type "Float (double-precision)") (DamageCauser :type "Actor Object Reference"))
  ; Take Damage
  (`self.OnFirstHit`)
  (set `self.currentHeathPoints` (`KismetMathLibrary.FMax` (- (`self.currentHeathPoints`) DamageAmount)))
  (`NiagaraFunctionLibrary.SpawnSystemAttached` "/Game/FX/Protagonist/Impact/NS_Impact.NS_Impact" (`self.mesh`) "None" (0.0 0.0 100.0) (struct) "SnapToTarget" true)
  (bind _healthbar (`self.healthBar`)
    (:`then`
      (`/Game/Entities/Player/VFX/WBP_HealthBar.SetFillLevel` _healthbar (/ (`self.currentHeathPoints`) (`self.maxHeathPoints`))))
    (:`else`
      _))
  (if (<= (`self.currentHeathPoints`) 0.0)
    (`self.Death` DamageCauser)))

(event `OnGroundHit`
  (params (HitComponent :type "PrimitiveComponent Object Reference") (OtherActor :type "Actor Object Reference") (OtherComp :type "PrimitiveComponent Object Reference") (NormalImpulse :type "Vector Structure") (Hit :type "HitResult Structure (by ref)"))
  (bind _returnvalue (`Actor.GetComponentByClass` (`self.characterActor`) "/Game/Entities/Player/AC_MaskDropSystem.AC_MaskDropSystem_C"))
  (bind _returnvalue_2 (- (`Actor.K2_GetActorLocation` (`self.characterActor`)) (`SceneComponent.RelativeLocation` (`self.mesh`))))
  (if (`|EnumEquality` (`PrimitiveComponent.GetCollisionObjectType` OtherComp) "ECC_WorldStatic")
    (if (`KismetSystemLibrary.IsValidClass` (`self.shatterAsset`)) :!label _label_2
      (`/Engine/EditorBlueprintResources/StandardMacros.DoOnce` false
        (:`Completed`
          ; Create Shatter Asset
          (bind _returnvalue_3 (`|SpawnActorFromClass` (`self.shatterAsset`) (`KismetMathLibrary.MakeTransform` _returnvalue_2) "Undefined" "MultiplyWithRoot" null null))
          (set `/Game/Entities/Player/VFX/BP_EnemyShatter.timeBeforeDestroy` (`self.timeBeforeDestroy`) _returnvalue_3)
          (bind _returnvalue_4 (`|SpawnActorFromClass` "/Engine/EditorResources/FieldNodes/FS_MasterField.FS_MasterField_C" (`KismetMathLibrary.MakeTransform` _returnvalue_2 (`KismetMathLibrary.MakeRotFromX` (`self.HitDirection`))) "Undefined" "MultiplyWithRoot" null null))
          (set `/Engine/EditorResources/FieldNodes/FS_MasterField.Radial Magnitude` 3000.0 _returnvalue_4)
          (set `/Engine/EditorResources/FieldNodes/FS_MasterField.DirectionalMagnitude` 50000.0 _returnvalue_4)
          (set `/Engine/EditorResources/FieldNodes/FS_MasterField.TorqueMult` 32.0 _returnvalue_4)
          (`/Engine/EditorResources/FieldNodes/FS_MasterField.CE_Trigger` _returnvalue_4)
          (`Actor.K2_DestroyActor` _returnvalue_4)
          (`|ExecutionSequence`
            (:`then_0`
              ; Mask Spawn
              (`/Engine/EditorBlueprintResources/StandardMacros.IsValid` _returnvalue
                (:`Is Valid`
                  (`/Game/Entities/Player/AC_MaskDropSystem.SpawnMask` _returnvalue (`Actor.K2_GetActorLocation` (`self.characterActor`))))))
            (:`then_1`
              (`Actor.K2_DestroyActor` (`self.characterActor`)))))))))

(event `StartDeath`
  (goto _label_2))

(event `SpawnHealthBar`
  (bind _characteractor (`self.characterActor`))
  ; HealthBar
  (if (`self.hasHealthBar`)
    (bind _returnvalue (`|CreateWidget` "/Game/Entities/Player/VFX/WBP_HealthBar.WBP_HealthBar_C"))
    (set `self.healthBar` _returnvalue)
    (bind _returnvalue_2 (`|AddComponentByClass` _characteractor "/Script/UMG.WidgetComponent" false (`KismetMathLibrary.MakeTransform` (`KismetMathLibrary.MakeVector` 0.0 0.0 (+ (`CapsuleComponent.CapsuleHalfHeight` (`Character.CapsuleComponent` _characteractor)) (`self.healthBarZ_Offset`))))))
    (`WidgetComponent.SetWidgetSpace` _returnvalue_2 "Screen")
    (`WidgetComponent.SetWidget` _returnvalue_2 (`self.healthBar`))
    (`WidgetComponent.SetDrawSize` _returnvalue_2 (`self.healthBarSize`))))

(fn `HitLocationToDirection`
  (params (Location :type "Vector Structure"))
  (returns (Direction :type "EDirection Enum"))
  (bind _characteractor (`self.characterActor`))
  (bind _returnvalue (`KismetMathLibrary.GetDirectionUnitVector` (`Actor.K2_GetActorLocation` _characteractor) Location))
  (if (<= (`KismetMathLibrary.DegAcos` (`KismetMathLibrary.Dot_VectorVector` _returnvalue (`Actor.GetActorForwardVector` _characteractor))) 45.0)
    (return "Front")
    (elif (<= (`KismetMathLibrary.DegAcos` (`KismetMathLibrary.Dot_VectorVector` _returnvalue (`KismetMathLibrary.NegateVector` (`Actor.GetActorForwardVector` _characteractor)))) 45.0)
      (return "Back")
      (elif (>= (`KismetMathLibrary.Dot_VectorVector` _returnvalue (`Actor.GetActorRightVector` _characteractor)) 0.0)
        (return "Right")
        (else
          (return "Left"))))))

(fn `IsTargetingPlayer ?`
  (returns (ReturnValue :type Boolean))
  (locals (AttackTarget :type Name :default "AttackTarget"))
  (return (== (`GameplayStatics.GetPlayerCharacter` 0) (`BlackboardComponent.GetValueAsObject` (`AIBlueprintHelperLibrary.GetBlackboard` (`self.GetOwner`)) (`local.AttackTarget`)))))

(fn `OnFirstHit`
  (locals (`Camera Index` :type Integer))
  (bind _returnvalue (`GameplayStatics.GetGameMode`))
  (cast `/Game/Entities/NPCs/Enemies/Elite/BP_Elite` (`self.GetOwner`)
    (:`then`
      (`|ExecutionSequence`
        (:`then_0`
          (bind _asgm_test (cast `/Game/Core/GameModes/Game/GM_Test` _returnvalue))
          (if (`/Game/Core/GameModes/Game/GM_Test.isInCombat` _asgm_test)
            (return)
            (else
              _)))
        (:`then_1`
          (bind _asgm_base (cast `/Game/Core/GameModes/Game/GM_Base` _returnvalue))
          (if (`/Game/Core/GameModes/Game/GM_Base.isInCombat` _asgm_base)
            (return)
            (else
              _))))
      (set `/Game/Core/GameModes/Game/GM_Test.isInCombat` true _asgm_test))
    (:`CastFailed`
      _))
  (`|ExecutionSequence`
    (:`then_0`
      (`self.SpawnHealthBar`))
    (:`then_1`
      ; Change Camera
      (`self.SetToStaticCamera`))
    (:`then_2`
      (if (not (`self.IsTargetingPlayer ?`))
        ; NPC Hit without detection
        (bind _asbp_elite (cast `/Game/Entities/NPCs/Enemies/Elite/BP_Elite` (`self.GetOwner`)))
        (`/Game/Entities/NPCs/Enemies/Elite/BP_Elite.GotFirstHit` _asbp_elite))
      (return))))