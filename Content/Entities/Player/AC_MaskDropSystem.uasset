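; Actor component that drops a mask pickup into the world on behalf of its owner.
; Its SpawnMask event checks that a MaskPickup profile is set, spawns a half-scale BP_MaskPickup at the given location and passes that profile to it.
; On BeginPlay it calls IsEnemyMessage on the owner through an interface, but nothing in the graph uses the result.
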(event `self.ReceiveBeginPlay`
  (bind _returnvalue (`self.GetOwner`))
  (if (`KismetSystemLibrary.DoesImplementInterface` _returnvalue)
    (bind _bp_enemy (message `/Game/Entities/Player/BPI_IsEnemy.IsEnemy` _returnvalue))))

(event `SpawnMask`
  (params (`Spawn Transform Location` :type "Vector Structure"))
  (bind _maskpickup (`self.maskPickup`)
    (:`then`
      (bind _returnvalue (`|SpawnActorFromClass` "/Game/Entities/Player/BP_MaskPickup.BP_MaskPickup_C" (`KismetMathLibrary.MakeTransform` `Spawn Transform Location` (struct) (0.5 0.5 0.5)) "Undefined" "MultiplyWithRoot" null null))
      (set `/Game/Entities/Player/BP_MaskPickup.maskProfile` _maskpickup _returnvalue))
    (:`else`)))