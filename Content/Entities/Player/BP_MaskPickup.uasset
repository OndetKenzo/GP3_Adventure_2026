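; BP_MaskPickup is a world pickup for a mask, previewed as the MaskProfile's mesh, or as a texture widget when no mesh is set.
; A looping timer and MaskRotationTimeline drive the preview rotation toward the player camera.
; On Box overlap, a tag and interface check identifies the player and passes the pickup to their AC_MaskSystem.
; A separate Pickup event destroys the actor.
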(event `self.ReceiveBeginPlay`
  (bind _maskmesh (`/Game/Entities/Player/PDA_MaskProfile.maskMesh` (`self.maskProfile`)))
  (`KismetSystemLibrary.Delay` 0.2)
  (bind _returnvalue (`|CreateWidget` "/Game/Entities/Player/VFX/WBP_MaskPreview.WBP_MaskPreview_C"))
  (`WidgetComponent.SetWidget` (`self.MaskPreview`) _returnvalue)
  (`/Game/Entities/Player/VFX/WBP_MaskPreview.SetMaskTexture` _returnvalue (`/Game/Entities/Player/PDA_MaskProfile.maskTexture` (`self.maskProfile`)))
  (`|ExecutionSequence`
    (:`then_0`
      (`/Engine/EditorBlueprintResources/StandardMacros.IsValid` _maskmesh
        (:`Is Valid`
          (`StaticMeshComponent.SetStaticMesh` (`self.MaskPreviewMesh`) _maskmesh))
        (:`Is Not Valid`
          (`SceneComponent.SetVisibility` (`self.MaskPreviewMesh`) false false)
          (`SceneComponent.SetVisibility` (`self.MaskPreview`) true false))))
    (:`then_1`
      (bind _returnvalue_2 (`KismetSystemLibrary.K2_SetTimerDelegate` (`|CreateDelegate` :!event `MaskRotation`) 1.0 true))
      (set `self.CameraRotationTimer` _returnvalue_2))))

(event `StopMaskRotation`
  (`KismetSystemLibrary.K2_ClearAndInvalidateTimerHandle` (`self.CameraRotationTimer`)))

(event `MaskRotation`
  (bind (_returnvalue_roll _returnvalue_pitch _returnvalue_yaw) (`KismetMathLibrary.BreakRotator` (`KismetMathLibrary.FindLookAtRotation` (`SceneComponent.K2_GetComponentLocation` (`self.MaskPreviewMesh`)) (`self.K2_GetActorLocation` (`GameplayStatics.GetPlayerCameraManager` 0)))))
  ; Rotate Preview Widget to Face Camera
  (`Timeline|MaskRotationTimeline` :!via `PlayFromStart`
    (:`Update`
      (`SceneComponent.K2_SetWorldRotation` :`self` (`self.Collision`))
      (`SceneComponent.K2_SetWorldRotation` (`self.MaskPreview`) (`KismetMathLibrary.FindLookAtRotation` (`SceneComponent.K2_GetComponentLocation` (`self.MaskPreview`)) (`self.K2_GetActorLocation` (`GameplayStatics.GetPlayerCameraManager` 0))) false false)
      (`SceneComponent.K2_SetWorldRotation` (`self.MaskPreviewMesh`) (`KismetMathLibrary.MakeRotator` _returnvalue_roll (+ _returnvalue_pitch -45.0) (+ _returnvalue_yaw -90.0)) false false))))

(event `self.Collision.OnComponentBeginOverlap`
  (params (OverlappedComponent :type "PrimitiveComponent Object Reference") (OtherActor :type "Actor Object Reference") (OtherComp :type "PrimitiveComponent Object Reference") (OtherBodyIndex :type Integer) (bFromSweep :type Boolean) (SweepResult :type "HitResult Structure (by ref)")))

(event `self.Box.OnComponentBeginOverlap`
  (params (OverlappedComponent :type "PrimitiveComponent Object Reference") (OtherActor :type "Actor Object Reference") (OtherComp :type "PrimitiveComponent Object Reference") (OtherBodyIndex :type Integer) (bFromSweep :type Boolean) (SweepResult :type "HitResult Structure (by ref)"))
  ; Pickup Logic
  (if (`ActorComponent.ComponentHasTag` OtherComp "PlayerCollision")
    (if (`KismetSystemLibrary.DoesImplementInterface` OtherActor "/Game/Entities/Player/BPI_IsPlayer.BPI_IsPlayer_C")
      (bind _bp_player (message `/Game/Entities/Player/BPI_IsPlayer.IsPlayer` OtherActor))
      (`/Game/Entities/Player/AC_MaskSystem.PickupMask` (`self.GetComponentByClass` _bp_player "/Game/Entities/Player/AC_MaskSystem.AC_MaskSystem_C") self))))

(event `Pickup`
  (`self.K2_DestroyActor`))

(fn `UserConstructionScript`)