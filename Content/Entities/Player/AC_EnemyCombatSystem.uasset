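; Actor component that handles enemy attack hit detection and damage for its owning Character.
; Hits come from sphere traces, either swept between two mesh sockets or run at a single given location.
; Each struck actor implementing BPI_IsPlayer, or BPI_IsEnemy when Friendlyfire is on, takes point damage.
; A HitActors list prevents repeat damage until ClearHitActors empties it.
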(event `self.ReceiveBeginPlay`
  (bind _ascharacter (cast `Character` (`self.GetOwner`)))
  (set `self.characterMesh` (`Character.Mesh` _ascharacter)))

(event `ClearHitActors`
  (`KismetArrayLibrary.Array_Clear` (`self.hitActors`)))

(event `TriggerHit`
  (params (DamageAmount :type "Float (double-precision)") (Radius :type "Float (single-precision)") (ObjectTypes :type "Array of EObjectTypeQuery Enum (by ref)") (StartSocket :type Name) (EndSocket :type Name))
  (bind (_startlocation _endlocation) (`self.FindHitLocation` StartSocket EndSocket))
  (bind (_outhits _returnvalue) (`KismetSystemLibrary.SphereTraceMultiForObjects` :`Start` _startlocation :`End` _endlocation :`Radius` Radius :`ObjectTypes` ObjectTypes :`DrawTime` 20.0))
  (`self.ApplyDamageToHitActors` DamageAmount _returnvalue _outhits))

(event `Trigger HitCapsule`
  (params (DamageAmount :type "Float (double-precision)") (Radius :type "Float (double-precision)") (ObjectTypes :type "Array of EObjectTypeQuery Enum (by ref)") (Location :type "Vector Structure"))
  (bind (_outhits _returnvalue) (`KismetSystemLibrary.SphereTraceMultiForObjects` Location Location Radius ObjectTypes))
  (`self.ApplyDamageToHitActors` DamageAmount _returnvalue _outhits))

(fn `ApplyDamageToHitActors`
  (params (Amount :type "Float (double-precision)") (Hit :type Boolean) (Hits :type "Array of HitResult Structure"))
  (locals (HitActor :type "Actor Object Reference") (HitResult :type "HitResult Structure"))
  (if Hit
    (for _array_element Hits
      (set `local.HitResult` _array_element)
      (set `local.HitActor` (`.HitActor` (`GameplayStatics.BreakHitResult` _array_element)))
      (if (not (`KismetArrayLibrary.Array_Contains` (`self.hitActors`) (`local.HitActor`)))
        (`|ExecutionSequence`
          (:`then_0`
            (if (`KismetSystemLibrary.DoesImplementInterface` (`local.HitActor`) "/Game/Entities/Player/BPI_IsPlayer.BPI_IsPlayer_C")
              (`GameplayStatics.ApplyPointDamage` (`local.HitActor`) (`local.Amount`) (0.0 0.0 0.0) (`local.HitResult`) :!label _label)
              (`KismetArrayLibrary.Array_Add` (`self.hitActors`) (`local.HitActor`))))
          (:`then_1`
            (if (`self.friendlyfire`)
              (if (`KismetSystemLibrary.DoesImplementInterface` (`local.HitActor`) "/Game/Entities/Player/BPI_IsEnemy.BPI_IsEnemy_C")
                (goto _label)))))))))

(fn `FindHitLocation`
  (params (StartSocket :type Name) (EndSocket :type Name))
  (returns (StartLocation :type "Vector Structure") (EndLocation :type "Vector Structure"))
  (bind _charactermesh (`self.characterMesh`))
  (bind _returnvalue (`Actor.K2_GetActorLocation` (`self.GetOwner`)))
  (`/Engine/EditorBlueprintResources/StandardMacros.IsValid` _charactermesh
    (:`Is Valid`
      (return (`SceneComponent.GetSocketLocation` _charactermesh StartSocket) (`SceneComponent.GetSocketLocation` _charactermesh EndSocket)))
    (:`Is Not Valid`
      (return _returnvalue _returnvalue))))