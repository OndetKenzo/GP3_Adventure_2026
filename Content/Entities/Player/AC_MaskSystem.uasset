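; Player component that handles picking up, equipping and persisting masks, plus narrative pickups.
; Pickups broadcast a dispatcher with the animation length as delay and play the pickup montage on the player's mesh.
; TakeMask saves the pending mask through GI_Main, broadcasts life, scale and speed updates, announces the mask and destroys the pickup.
; LoadMask only rebroadcasts the saved mask through OnTakeMask, without applying stats itself.
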(event `PickupNarratif`
  (params (NarratifProfile :type "/Game/Entities/Player/PDA_NarratifProfile Object Reference"))
  (`self.OnPickupNarratif` NarratifProfile (`AnimSequenceBase.SequenceLength` (`self.pickupAnim`)))
  (`self.PlayPickupAnim`))

(event `PlayPickupAnim`
  (bind _returnvalue (`self.GetOwner`))
  ; Pickup Animation
  (if (`KismetSystemLibrary.DoesImplementInterface` _returnvalue "/Game/Entities/Player/BPI_IsPlayer.BPI_IsPlayer_C")
    (bind _bp_player (message `/Game/Entities/Player/BPI_IsPlayer.IsPlayer` _returnvalue))
    (`|PlayMontage` (`Character.Mesh` _bp_player) (`self.pickupAnim`))))

(event `PickupMask`
  (params (MaskPickup :type "/Game/Entities/Player/BP_MaskPickup Object Reference"))
  (bind _output_get (set `self.tempMask` MaskPickup))
  (`self.OnPickupMask` (`/Game/Entities/Player/BP_MaskPickup.maskProfile` _output_get) (`AnimSequenceBase.SequenceLength` (`self.pickupAnim`)))
  (`self.PlayPickupAnim`))

(event `TakeMask`
  (bind _tempmask (`self.tempMask`))
  (bind _maskprofile (`/Game/Entities/Player/BP_MaskPickup.maskProfile` _tempmask))
  (set `self.currentMask` _maskprofile)
  (`self.SaveMask` _maskprofile)
  (`self.SetMaskStats` _maskprofile)
  (`self.OnTakeMask` _maskprofile)
  (`Actor.K2_DestroyActor` _tempmask))

(event `SetMaskStats`
  (params (currentMask :type "/Game/Entities/Player/PDA_MaskProfile Object Reference"))
  (bind _currentmask (`self.currentMask`))
  (bind (_value _returnvalue) (`BlueprintMapLibrary.Map_Find` (`/Game/Entities/Player/PDA_MaskProfile.maskEffect` currentMask) "NewEnumerator3"))
  ; Set Player Stats
  (`|ExecutionSequence`
    (:`then_0`
      (`self.SetLife` (`/Game/Entities/Player/PDA_MaskProfile.hp` _currentmask) (`/Game/Entities/Player/PDA_MaskProfile.maskPieces` _currentmask)))
    (:`then_1`
      (if _returnvalue
        (`self.SetScale` _value)
        (else
          (`self.SetScale` 1.0))))
    (:`then_2`
      (`self.SetSpeed`))))

(fn `LoadMask`
  ; Load And Apply mask save
  (bind _asgi_main (cast `/Game/Core/Saves/GI_Main` (`GameplayStatics.GetGameInstance`)))
  (bind _sgb_game (`/Game/Core/Saves/GI_Main.LoadGame` _asgi_main))
  (`self.OnTakeMask` (`/Game/Core/Saves/SGB_Game.currentMask` _sgb_game)))

(fn `SaveMask`
  (params (MaskProfile :type "/Game/Entities/Player/PDA_MaskProfile Object Reference"))
  (bind _asgi_main (cast `/Game/Core/Saves/GI_Main` (`GameplayStatics.GetGameInstance`)))
  (`/Game/Core/Saves/GI_Main.SaveMask` _asgi_main MaskProfile))