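; Player health component that handles damage, healing, death and respawn for BP_Player, broadcasting dispatchers for UI and game logic.
; Point damage is diverted to parry feedback and an optional enemy stun while parrying, otherwise it passes god mode and i-frame checks.
; Valid hits grant i-frames and play hurt sound and montage, with death refilling health.
; Input actions toggle god mode and cheat-heal.
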(event `self.ReceiveBeginPlay`
  (bind _asgm_base (cast `/Game/Core/GameModes/Game/GM_Base` (`GameplayStatics.GetGameMode`)))
  (add `/Game/Core/GameModes/Game/GM_Base.OnRespawn` _asgm_base (delegate `ResetHealth`))
  (bind _asbp_player (cast `/Game/Entities/Player/BP_Player` (`self.GetOwner`)))
  (bind _output_get (set `self.player` _asbp_player))
  (set `self.playerParrySystem` (`Actor.GetComponentByClass` _output_get "/Game/Entities/Player/PlayerCombatSystem/AC_ParrySystem.AC_ParrySystem_C"))
  (add `Actor.OnTakePointDamage` _output_get (`|CreateDelegate` :!event `OnTakePointDamage_Event`))
  (set `self.currentHeathPoints` (`self.maxHeathPoints`)))

(event `ResetHealth`
  (bind _maxheathpoints (`self.maxHeathPoints`))
  (`self.OnHeal` _maxheathpoints _maxheathpoints))

(event `OnTakePointDamage_Event`
  (params (DamagedActor :type "Actor Object Reference") (Damage :type "Float (single-precision)") (InstigatedBy :type "Controller Object Reference") (HitLocation :type "Vector Structure") (FHitComponent :type "PrimitiveComponent Object Reference") (BoneName :type Name) (ShotFromDirection :type "Vector Structure") (DamageType :type "DamageType Object Reference") (DamageCauser :type "Actor Object Reference"))
  (bind _returnvalue (`Actor.GetComponentByClass` (`self.player`) "/Game/Entities/Player/PlayerCombatSystem/AC_ParrySystem.AC_ParrySystem_C"))
  (bind _ac_parrysystem (`/Game/Entities/Player/BP_Player.AC_ParrySystem` (`self.player`)))
  (if (not (`/Game/Entities/Player/PlayerCombatSystem/AC_ParrySystem.isParrying` (`self.playerParrySystem`)))
    (`self.ProcessDamage` (`KismetMathLibrary.FTrunc` Damage))
    (else
      ; Parry Juice
      (`/Engine/EditorBlueprintResources/StandardMacros.IsValid` _returnvalue
        (:`Is Valid`
          (`/Game/Entities/Player/PlayerCombatSystem/AC_PlayerCombatSystem.ActionJuice` :`self` _returnvalue)
          (`self.OnParry`)
          ; Stun On Parry
          (if (`/Game/Entities/Player/PlayerCombatSystem/AC_ParrySystem.stunOnParry` _ac_parrysystem)
            (if (`KismetSystemLibrary.DoesImplementInterface` DamageCauser "/Game/Entities/Player/BPI_IsEnemy.BPI_IsEnemy_C")
              (message `/Game/Entities/Player/BPI_IsEnemy.SetStunState` DamageCauser (`/Game/Entities/Player/PlayerCombatSystem/AC_ParrySystem.stunOnParryDuration` _ac_parrysystem)))))))))

(event `ProcessDamage`
  (params (DamageAmount :type Integer))
  (if (`self.godmode`)
    (`self.OnGodMode`)
    (elif (not (> (`/Game/Entities/Player/BP_Player.iFrameTimer` (`self.player`)) 0))
      (set `self.currentHeathPoints` (`KismetMathLibrary.Max` (- (`self.currentHeathPoints`) DamageAmount)))
      ; Hurt Juice
      (`|ExecutionSequence`
        (:`then_0`
          (if (not (<= (`self.currentHeathPoints`) 0))
            (`/Game/Entities/Player/BP_Player.iFrame` (`self.player`) (`self.iFrameDuration`))))
        (:`then_1`
          (`GameplayStatics.PlaySoundAtLocation` "/Game/Placeholder/SFX/SC_Hurt.SC_Hurt" (`Actor.K2_GetActorLocation` (`self.player`)) (struct) 1.0 1.0 0.0 null null null null)
          (`|PlayMontage` (`Character.Mesh` (`self.player`)) (`self.hitReactAnimations`)
            (:`then`
              ;; HealthBar
              (`self.OnDamage` (`self.currentHeathPoints`) (`self.maxHeathPoints`))
              (if (<= (`self.currentHeathPoints`) 0.0)
                (`|PlayMontage` (`Character.Mesh` (`self.player`)) (`self.deathAnimations`)
                  (:`then`
                    (`self.OnDeath`)
                    (set `self.currentHeathPoints` (`self.maxHeathPoints`))))))))))))

(event `Heal`
  (params (Amount :type Integer))
  (set `self.currentHeathPoints` (`KismetMathLibrary.Min` (+ (`self.currentHeathPoints`) Amount) (`self.maxHeathPoints`)))
  (`self.OnHeal` (`self.currentHeathPoints`) (`self.maxHeathPoints`)))

(event `EnhancedInput|/Game/Core/Inputs/Actions/IA_Godmode`
  (params (ActionValue :type Boolean) (ElapsedSeconds :type "Float (double-precision)") (TriggeredSeconds :type "Float (double-precision)") (InputAction :type "InputAction Object Reference" :default "/Game/Core/Inputs/Actions/IA_Godmode.IA_Godmode"))
  (:`Started`
    (`/Engine/EditorBlueprintResources/StandardMacros.FlipFlop`
      (:`A`
        (set `self.godmode` true)
        (`self.OnGodMode`)
        (`KismetSystemLibrary.PrintString` "god mode on" true true (struct :`R` 1.0 :`G` 0.904903 :`A` 1.0)))
      (:`B`
        (set `self.godmode` false)
        (`KismetSystemLibrary.PrintString` "god mode off" true true (struct :`R` 1.0 :`G` 0.013814 :`A` 1.0))))))

(event `EnhancedInput|/Game/Core/Inputs/Actions/IA_CheatHeal`
  (params (ActionValue :type Boolean) (ElapsedSeconds :type "Float (double-precision)") (TriggeredSeconds :type "Float (double-precision)") (InputAction :type "InputAction Object Reference" :default "/Game/Core/Inputs/Actions/IA_CheatHeal.IA_CheatHeal"))
  (:`Started`
    (`self.Heal` 1)))