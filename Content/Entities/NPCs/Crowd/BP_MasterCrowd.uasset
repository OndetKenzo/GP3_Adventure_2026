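; Base crowd NPC that gives itself a random skeletal mesh and data-table-driven color variations on BeginPlay.
; It registers with the Animation Sharing manager on the popcorn skeleton, with GetCrowdState resolving on-demand versus current animation states.
; Player parry, win and combo events set CrowdState by crowd option (Neutral idles, Expressive reacts), while movement toggles a moving state.
; CrowdAgent supplies movement updates and position reset; BP_CrowdManager handles unloading.
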(event `self.ReceiveBeginPlay`
  ; To remove
  (`parent.ReceiveBeginPlay`)
  (`KismetSystemLibrary.DelayUntilNextTick`)
  (bind _returnvalue (`GameplayStatics.GetActorOfClass` "/Game/Entities/NPCs/Crowd/BP_CrowdManager.BP_CrowdManager_C"))
  (`self.SetCrowdAgent` _returnvalue)
  (`SkeletalMeshComponent.SetSkeletalMeshAsset` (`self.Mesh`) (`KismetArrayLibrary.Array_Random` (`self.Skeletal_Crowd`)))
  (for (_array_element _array_index) (`MeshComponent.GetMaterials` (`self.Mesh`))
    (bind _returnvalue_2 (`KismetMaterialLibrary.CreateDynamicMaterialInstance` _array_element))
    (`PrimitiveComponent.SetMaterial` (`self.Mesh`) _array_index _returnvalue_2)
    (bind _output (`self.RandomFromTable` "/Game/Data/Tables/T_SingleColors1.T_SingleColors1"))
    (bind _returnvalue_3 (`|GetDataTableRow` "/Game/Data/Tables/T_SingleColors1.T_SingleColors1" _output)
      (:`then`
        (`MaterialInstanceDynamic.SetVectorParameterValue` _returnvalue_2 "Color_Variation_01" (`KismetMathLibrary.Conv_ColorToLinearColor` (break `/Game/Data/Structs/S_SingleColor` _returnvalue_3)))
        (bind _output_2 (`self.RandomFromTable` "/Game/Data/Tables/T_SingleColors2.T_SingleColors2"))
        (bind _returnvalue_4 (`|GetDataTableRow` "/Game/Data/Tables/T_SingleColors2.T_SingleColors2" _output_2)
          (:`then`
            (`MaterialInstanceDynamic.SetVectorParameterValue` _returnvalue_2 "Color_Variation_02" (`KismetMathLibrary.Conv_ColorToLinearColor` (break `/Game/Data/Structs/S_SingleColor` _returnvalue_4)))
            (bind _output_3 (`self.RandomFromTable` "/Game/Data/Tables/T_SingleColors3.T_SingleColors3"))
            (bind _returnvalue_5 (`|GetDataTableRow` "/Game/Data/Tables/T_SingleColors3.T_SingleColors3" _output_3)
              (:`then`
                (`MaterialInstanceDynamic.SetVectorParameterValue` _returnvalue_2 "Color_Variation_03" (`KismetMathLibrary.Conv_ColorToLinearColor` (break `/Game/Data/Structs/S_SingleColor` _returnvalue_5)))))))))))

(event `BindCrowdEvent`
  ; To remove
  (add `CrowdAgentComponent.OnMovementUpdate` (`self.CrowdAgent`) (`|CreateDelegate` :!event `PlayerMoving`)))

(event `PlayerPary`
  ; Favour Player
  (switch `/Game/Entities/NPCs/Crowd/AnimationSharing/E_CrowdOpinion` (`self.CrowdOption`)
    (:`NewEnumerator0`
      (`self.SetRandomIdleState`))
    (:`NewEnumerator1`
      (set `self.CrowdState` "NewEnumerator2"))))

(event `PlayerWin`
  ; Favour Player
  (switch `/Game/Entities/NPCs/Crowd/AnimationSharing/E_CrowdOpinion` (`self.CrowdOption`)
    (:`NewEnumerator0`
      (`self.SetRandomIdleState`))
    (:`NewEnumerator1`
      (set `self.CrowdState` "NewEnumerator5"))))

(event `PlayerCombot`
  ; Favour Player
  (switch `/Game/Entities/NPCs/Crowd/AnimationSharing/E_CrowdOpinion` (`self.CrowdOption`)
    (:`NewEnumerator0`
      (`self.SetRandomIdleState`))
    (:`NewEnumerator1`
      (set `self.CrowdState` "NewEnumerator3"))))

(event `PlayerMoving`
  (params (bIsMoving :type Boolean))
  (if bIsMoving
    (set `self.CrowdState` "NewEnumerator8")
    (else
      (`self.SetRandomIdleState`))))

(fn `GetCrowdState`
  (params (OnDemandeState :type Byte) (CurrentState :type Byte))
  (returns (State :type "/Game/Entities/NPCs/Crowd/AnimationSharing/E_CrowdState Enum"))
  (if (!= OnDemandeState 255)
    (`self.IsOnDemand`
      (:`then`
        _)
      (:`else`
        (set `self.IsOnDemand` true)))
    (return (`self.CrowdState`))
    (elif (`self.IsOnDemand`)
      (set `self.IsOnDemand` false)
      (bind _output_get (set `self.CrowdState` (cast `/Game/Entities/NPCs/Crowd/AnimationSharing/E_CrowdState` (`local.CurrentState`))))
      (return _output_get)
      (else
        (return (`self.CrowdState`))))))

(fn `GetMesh`)

(fn `RandomFromTable`
  (params (Table :type "DataTable Object Reference"))
  (returns (Output :type "Name (by ref)"))
  (bind _outrownames (`DataTableFunctionLibrary.GetDataTableRowNames` Table))
  (return (`|GetArrayItem` _outrownames (`KismetMathLibrary.RandomInteger` (`KismetArrayLibrary.Array_Length` _outrownames)))))

(fn `ReleaseAgent`
  (bind _returnvalue (`GameplayStatics.GetActorOfClass` "/Game/Entities/NPCs/Crowd/BP_CrowdManager.BP_CrowdManager_C"))
  (`/Game/Entities/NPCs/Crowd/BP_CrowdManager.UnloadActor` _returnvalue self))

(fn `ResetPos`
  (`CrowdAgentComponent.ResetOriginalLocation` (`self.CrowdAgent`)))

(fn `SetCrowdAgent`
  (params (CrowdManager :type "/Game/Entities/NPCs/Crowd/BP_CrowdManager Object Reference"))
  (bind _returnvalue (`AnimationSharingManager.GetAnimationSharingManager`))
  (`AnimationSharingManager.RegisterActorWithSkeletonBP` _returnvalue self "/Game/Entities/Character/Mesh/Popcorn/SK_Popcorn_Skeleton.SK_Popcorn_Skeleton")
  (`self.BindCrowdEvent`)
  (`self.SetRandomIdleState`))

(fn `SetRandomIdleState`
  (set `self.CrowdState` "NewEnumerator14")
  (return))

(fn `UserConstructionScript`)