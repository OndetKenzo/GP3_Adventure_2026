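; Manager for crowd NPCs that react to the player's combat, using an Animation Sharing manager created at BeginPlay.
; Registered NPCs get one of two random crowd options against a Neutral threshold.
; Player parry and combo events post a bark sound and trigger each member's parry reaction; the damage handler has no reaction yet.
; It releases members before level loading and has actor-pool helpers, including an unused render, screen and line-of-sight visibility check.
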(event `self.ReceiveBeginPlay`
  (`AnimationSharingManager.CreateAnimationSharingManager` "/Game/Entities/NPCs/Enemies/BP/AnimationSharing/AS_CrowdBoss.AS_CrowdBoss")
  (bind _asbp_player (cast `/Game/Entities/Player/BP_Player` (`GameplayStatics.GetPlayerCharacter` 0)))
  ; BindPlayerEvent
  (add `/Game/Entities/Player/BP_Player.OnDamage` _asbp_player (`|CreateDelegate` :!event `PlayerTakeDamage`))
  (add `/Game/Entities/Player/BP_Player.OnParry` _asbp_player (`|CreateDelegate` :!event `PlayerParry`))
  (add `/Game/Entities/Player/BP_Player.OnCombot` _asbp_player (`|CreateDelegate` :!event `OnCombot`)))

(event `AddCrowdNPC`
  (params (NPC :type "/Game/Entities/NPCs/Crowd/BP_MasterCrowd Object Reference"))
  ; ADD new Npc
  (`KismetArrayLibrary.Array_Add` (`self.CrowdMembers`) NPC)
  (`self.EvaluateCrowdReaction` NPC))

(event `PlayerParry`
  (`AkGameplayStatics.PostEvent` "/Game/WwiseAudio/Events/Default_Work_Unit/VOICES/Play_Barks_Waow.Play_Barks_Waow")
  (for _array_element (`self.CrowdMembers`)
    (`/Engine/EditorBlueprintResources/StandardMacros.IsValid` _array_element
      (:`Is Valid`
        (`/Game/Entities/NPCs/Crowd/BP_MasterCrowd.PlayerPary` _array_element)))))

(event `PlayerTakeDamage`
  (for _array_element (`self.CrowdMembers`)
    (`/Engine/EditorBlueprintResources/StandardMacros.IsValid` _array_element)))

(event `ReleaseAgentBefordLevelLoading`
  (bind _crowdmembers (`self.CrowdMembers`))
  (for _array_element _crowdmembers
    (`/Game/Entities/NPCs/Crowd/BP_MasterCrowd.ReleaseAgent` _array_element))
  (`KismetArrayLibrary.Array_Clear` _crowdmembers))

(event `OnCombot`
  (`AkGameplayStatics.PostEvent` "/Game/WwiseAudio/Events/Default_Work_Unit/VOICES/Play_Barks_Waow.Play_Barks_Waow")
  (for _array_element (`self.CrowdMembers`)
    (`/Engine/EditorBlueprintResources/StandardMacros.IsValid` _array_element
      (:`Is Valid`
        (`/Game/Entities/NPCs/Crowd/BP_MasterCrowd.PlayerPary` _array_element)))))

(fn `CheckVisibility`
  (params (Npc :type "/Game/Entities/NPCs/Crowd/BP_MasterCrowd Object Reference"))
  (returns (Visibility :type Boolean))
  ; If it was not render then actor is not visible and can be push in the pool
  (if (`self.WasRecentlyRendered` Npc 0.2)
    (bind _isonscreen (`self.IsLocationOnScreen` (`self.K2_GetActorLocation` Npc)))
    (if _isonscreen
      (bind _isinsight (`self.InLineOfSight` (0.0 0.0 0.0)))
      (if _isinsight
        (return true)
        (else
          _))))
  (`ActorPoolComponent.Push` (`self.ActorPool`) Npc)
  (return false))

(fn `EvaluateCrowdReaction`
  (params (CurrentNPC :type "/Game/Entities/NPCs/Crowd/BP_MasterCrowd Object Reference"))
  (locals (Roll :type "Float (double-precision)" :default 0.0) (Neutral :type "Float (double-precision)" :default 0.2) (FavorPlayer :type "Float (double-precision)" :default 0.6))
  (set `local.Roll` (`KismetMathLibrary.RandomFloatInRange` 0.0 1.0))
  (if (< (`local.Roll`) (`local.Neutral`))
    (bind _currentnpc (`local.CurrentNPC`)
      (:`then`
        (set `/Game/Entities/NPCs/Crowd/BP_MasterCrowd.CrowdOption` "NewEnumerator0" _currentnpc)
        (return))
      (:`else`))
    (else
      (bind _currentnpc_2 (`local.CurrentNPC`)
        (:`then`
          (set `/Game/Entities/NPCs/Crowd/BP_MasterCrowd.CrowdOption` "NewEnumerator1" _currentnpc_2)
          (return))
        (:`else`)))))

(fn `GetActorToSpawn`
  (returns (ActorToSpawn :type "/Game/Entities/NPCs/Crowd/BP_MasterCrowd Object Reference"))
  (locals (ListActor :type "Array of /Game/Entities/NPCs/Crowd/BP_MasterCrowd Class Reference"))
  (bind _returnvalue (`ActorPoolComponent.Pull` (`self.ActorPool`)))
  (bind _asbp_master_crowd (cast `/Game/Entities/NPCs/Crowd/BP_MasterCrowd` _returnvalue))
  (return _asbp_master_crowd))

(fn `GetCrowdState`
  (returns (State :type "/Game/Entities/NPCs/Crowd/AnimationSharing/E_CrowdState Enum"))
  (return "NewEnumerator0"))

(fn `InLineOfSight`
  (params (WorldPosition :type "Vector Structure") (Actor :type "Actor Object Reference"))
  (returns (IsInSight :type Boolean))
  (bind _returnvalue (`GameplayStatics.GetPlayerController` 0))
  (bind _outhit (`KismetSystemLibrary.LineTraceSingle` (`PlayerCameraManager.GetCameraLocation` (`PlayerController.PlayerCameraManager` _returnvalue)) WorldPosition "TraceTypeQuery3" false (`|MakeArray` _returnvalue :!type "Actor Object Reference")))
  (return (== (`.HitActor` (`GameplayStatics.BreakHitResult` _outhit)) Actor)))

(fn `IsLocationOnScreen`
  (params (WorldPosition :type "Vector Structure"))
  (returns (IsOnScreen :type Boolean))
  (bind _returnvalue (`GameplayStatics.GetPlayerController` 0))
  (bind _screenposition (`GameplayStatics.ProjectWorldToScreen` _returnvalue WorldPosition))
  (bind (_sizex _sizey) (`PlayerController.GetViewportSize` _returnvalue))
  (bind _returnvalue_2 (/ (`KismetMathLibrary.BreakVector2D` _screenposition) _sizex))
  (bind _returnvalue_3 (/ (`.Y` (`KismetMathLibrary.BreakVector2D` _screenposition)) _sizey))
  (return (and (> _returnvalue_2 0.0) (< _returnvalue_2 1.0) (> _returnvalue_3 0.0) (< _returnvalue_3 1.0))))

(fn `UnloadActor`
  (params (Actor :type "/Game/Entities/NPCs/Crowd/BP_MasterCrowd Object Reference"))
  (`ActorPoolComponent.Push` (`self.ActorPool`) Actor))

(fn `UserConstructionScript`)