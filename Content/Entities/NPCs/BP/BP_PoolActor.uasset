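; BP_PoolActor is a poolable actor for NPC entities that switches between in-use and dormant states rather than being spawned or destroyed.
; GetItem and ReturnItem events call SetInUse with true and false respectively.
; SetInUse toggles collision, visibility and actor tick together, then stores the state in InUse.
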(event `GetItem`
  (`self.SetInUse` true))

(event `ReturnItem`
  (`self.SetInUse` false))

(fn `SetInUse`
  (params (value :type Boolean))
  (`self.SetActorEnableCollision` value)
  (`self.SetActorHiddenInGame` (not (`local.value`)))
  (`self.SetActorTickEnabled` (`local.value`))
  (set `self.InUse` (`local.value`)))

(fn `UserConstructionScript`)