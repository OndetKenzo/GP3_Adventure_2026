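; BP_Zone is a zone actor that makes the crowd form a circle around its sphere, for arenas or timed shots.
; TriggerArena forms the circle and starts an Elite discovery Level Sequence, while BreakArena releases it and TriggerShot adds duration and random offsets.
; The sequence is spawned at runtime, moved to the player pawn's transform and bound to the Elite by tag.
; When it finishes, the Elite changes skin.
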(event `EliteDiscoverSequence`
  (params (Elite :type "/Game/Entities/NPCs/Enemies/Elite/BP_Elite Object Reference"))
  (bind _sequenceplayer (`LevelSequenceActor.SequencePlayer` (`self.LevelSequence`)))
  (set `self.Elite` Elite)
  (bind _outactor (`LevelSequencePlayer.CreateLevelSequencePlayer` (`self.AnimEliteDiscover`) (make `MovieSceneSequencePlaybackSettings` false (struct) (struct :`bAllowRounding` true) 1.0 0.0 false true true false true)))
  (set `self.LevelSequence` _outactor)
  (`|ExecutionSequence`
    (:`then_0`
      ; Repositionning level sequence
      (set `LevelSequenceActor.bOverrideInstanceData` true (`self.LevelSequence`))
      (`self.K2_SetActorTransform` (`self.LevelSequence`) (`self.GetTransform` (`GameplayStatics.GetPlayerPawn` 0)) false true))
    (:`then_1`
      (`LevelSequenceActor.SetBindingByTag` (`self.LevelSequence`) "Elite" (`|MakeArray` Elite :!type "Actor Object Reference") false))
    (:`then_2`
      (`MovieSceneSequencePlayer.Play` _sequenceplayer)
      (add `MovieSceneSequencePlayer.OnFinished` _sequenceplayer (delegate `ChangeEliteskin`)))))

(event `ChangeEliteskin`
  (`/Game/Entities/NPCs/Enemies/Elite/BP_Elite.ChangeSkin` (`self.Elite`)))

(fn `BreakArena`
  (`CrowdSubsystem.BreakCircle` (subsystem `CrowdSubsystem`)))

(fn `TriggerArena`
  (params (Elite :type "/Game/Entities/NPCs/Enemies/Elite/BP_Elite Object Reference"))
  (`self.EliteDiscoverSequence` Elite)
  (`CrowdSubsystem.FormCircle` (subsystem `CrowdSubsystem`) (`self.K2_GetActorLocation`) (`SphereComponent.GetScaledSphereRadius` (`self.Sphere`)) 0.0 1.0 1.0))

(fn `TriggerShot`
  (`CrowdSubsystem.FormCircle` (subsystem `CrowdSubsystem`) (`self.K2_GetActorLocation`) (`SphereComponent.GetScaledSphereRadius` (`self.Sphere`)) (`self.Duration`) (`self.MinOffset`) (`self.MaxOffset`)))

(fn `UserConstructionScript`)