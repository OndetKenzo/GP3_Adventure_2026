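; AI controller for the physics test NPCs that sends its controlled pawn toward a target actor.
; On possess, it copies the Target from the pawn, which is either a BP_NPCTest_Physics or a BP_NPCTest_Physics_Moving.
; BeginPlay calls MoveNPC, which issues a single AI MoveTo toward that Target if it is valid.
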(event `self.ReceivePossess`
  (params (PossessedPawn :type "Pawn Object Reference"))
  (bind _asbp_npctest_physics (cast `/Game/Entities/NPCs/BP/Physics/BP_NPCTest_Physics` PossessedPawn)
    (:`then`
      (set `self.Target` (`/Game/Entities/NPCs/BP/Physics/BP_NPCTest_Physics.Target` _asbp_npctest_physics)))
    (:`CastFailed`
      (bind _asbp_npctest_physics_moving (cast `/Game/Entities/NPCs/BP/Physics/BP_NPCTest_Physics_Moving` PossessedPawn))
      (set `self.Target` (`/Game/Entities/NPCs/BP/Physics/BP_NPCTest_Physics_Moving.Target` _asbp_npctest_physics_moving)))))

(event `self.ReceiveBeginPlay`
  (`self.MoveNPC`))

(event `MoveNPC`
  (bind _target (`self.Target`))
  (`/Engine/EditorBlueprintResources/StandardMacros.IsValid` _target
    (:`Is Valid`
      (`|AIMoveTo` (`self.K2_GetPawn`) (0.0 0.0 0.0) _target))))

(fn `UserConstructionScript`)