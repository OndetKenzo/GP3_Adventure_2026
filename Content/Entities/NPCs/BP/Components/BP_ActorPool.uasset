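; BP_ActorPool is an object pool that hands out reusable actors of a configured class.
; GetPoolItem reuses the first pooled actor not in use, or spawns and adds one on demand until the pool reaches its size limit.
; When the pool is full, it prints a message and reports failure.
; Pooled actors handle their own checkout and release through GetItem and ReturnItem, which the pool calls.
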(fn `GetAvailableActor`
  (returns (Actor :type "/Game/Entities/NPCs/BP/BP_PoolActor Object Reference"))
  (for _array_element (`self.Pool`)
    (if (not (`/Game/Entities/NPCs/BP/BP_PoolActor.InUse` _array_element))
      (return _array_element))))

(fn `GetPoolItem`
  (returns (Success :type Boolean) (Actor :type "/Game/Entities/NPCs/BP/BP_PoolActor Object Reference"))
  (locals (PoolActor :type "/Game/Entities/NPCs/BP/BP_PoolActor Object Reference"))
  (bind _poolactor (`local.PoolActor`))
  (bind _actor (`self.GetAvailableActor`))
  (`/Engine/EditorBlueprintResources/StandardMacros.IsValid` _actor
    (:`Is Valid`
      (`/Game/Entities/NPCs/BP/BP_PoolActor.GetItem` _actor)
      (return true _actor))
    (:`Is Not Valid`
      (if (< (`KismetArrayLibrary.Array_Length` (`self.Pool`)) (`self.PoolSize`))
        ; Add New item to the pool
        (bind _returnvalue (`|SpawnActorFromClass` (`self.PoolActorClass`) (`KismetMathLibrary.MakeTransform` (0.0 0.0 0.0)) "Undefined" "MultiplyWithRoot" null null))
        (bind _output_get (set `local.PoolActor` _returnvalue))
        (`/Engine/EditorBlueprintResources/StandardMacros.IsValid` _output_get
          (:`Is Valid`
            (`KismetArrayLibrary.Array_AddUnique` (`self.Pool`) _output_get)
            (`/Game/Entities/NPCs/BP/BP_PoolActor.GetItem` _poolactor)
            (return true _poolactor))
          (:`Is Not Valid`
            _))
        (else
          (`KismetSystemLibrary.PrintString` "Pool is Full")))
      (return false null))))

(fn `ReturnItem`
  (params (Actor :type "/Game/Entities/NPCs/BP/BP_PoolActor Object Reference"))
  (`/Game/Entities/NPCs/BP/BP_PoolActor.ReturnItem` Actor))

(fn `UserConstructionScript`)