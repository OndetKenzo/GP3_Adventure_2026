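; BP_MultiPool is an object pool manager that hands out and recycles actors of any requested class.
; GetItemOfClass looks up a BP_ActorPool for the class in a map, lazily spawning and registering one with the shared pool size when none exists, then returns an item from it.
; ReturnItem routes an actor back to the pool keyed by its class, and does nothing if no such pool exists.
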(fn `GetItemOfClass`
  (params (Class :type "/Game/Entities/NPCs/BP/BP_PoolActor Class Reference"))
  (returns (Success :type Boolean) (Actor :type "/Game/Entities/NPCs/BP/BP_PoolActor Object Reference"))
  (bind (_value _returnvalue) (`BlueprintMapLibrary.Map_Find` (`self.Pools`) Class))
  (if _returnvalue
    (bind (_success _actor) (`/Game/Entities/NPCs/BP/Components/BP_ActorPool.GetPoolItem` _value))
    (return _success _actor)
    (else
      (bind _returnvalue_2 (`|SpawnActorFromClass` "/Game/Entities/NPCs/BP/Components/BP_ActorPool.BP_ActorPool_C" (`KismetMathLibrary.MakeTransform` (0.0 0.0 0.0)) "Undefined" "MultiplyWithRoot" null null))
      (set `/Game/Entities/NPCs/BP/Components/BP_ActorPool.PoolSize` (`self.PoolSizes`) _returnvalue_2)
      (set `/Game/Entities/NPCs/BP/Components/BP_ActorPool.PoolActorClass` (`local.Class`) _returnvalue_2)
      (`BlueprintMapLibrary.Map_Add` (`self.Pools`) (`local.Class`) _returnvalue_2)
      (bind (_success_2 _actor_2) (`/Game/Entities/NPCs/BP/Components/BP_ActorPool.GetPoolItem` _returnvalue_2))
      (return _success_2 _actor_2))))

(fn `ReturnItem`
  (params (PoolItem :type "/Game/Entities/NPCs/BP/BP_PoolActor Object Reference"))
  (bind (_value _returnvalue) (`BlueprintMapLibrary.Map_Find` (`self.Pools`) (`GameplayStatics.GetObjectClass` PoolItem)))
  (if _returnvalue
    (`/Game/Entities/NPCs/BP/Components/BP_ActorPool.ReturnItem` _value (`local.PoolItem`))))

(fn `UserConstructionScript`)