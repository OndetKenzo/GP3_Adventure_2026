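; Elite enemy NPC that spawns with a random crowd mesh and turns into an arena fight once hit, with a separate event to swap in its elite skin.
; On begin play it feeds its detail actions to the attack component; the first hit plays an attack montage and targets the player through the blackboard.
; It triggers its combat zone once, teleporting the player there, and death breaks the arena.
; Static camera switching is disconnected.
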(event `self.ReceiveBeginPlay`
  (set `/Game/Entities/NPCs/Enemies/BP/Components/BPC_EnemyAttack.Actions` (`/Game/Data/DataAsset/PDA_EnemyAi.Actions` (`self.EliteDetails`)) (`self.BPC_EliteAttack`))
  (`/Game/Entities/NPCs/Enemies/BP/Components/BPC_EnemyAttack.CreateCooldownTable` (`self.BPC_EliteAttack`))
  (`SkeletalMeshComponent.SetSkeletalMeshAsset` (`self.Mesh`) (`KismetArrayLibrary.Array_Random` (`self.Skeletal_Crowd`))))

(event `GotFirstHit`
  (`self.GotFound`)
  (`self.triggercombactZone`))

(event `self.AC_EnemyHealthSystem.SetToStaticCamera`
  ; Camera set up
)

(event `self.AC_EnemyHealthSystem.ReturnToMainCamera`
  ; Camera set up
)

(event `triggercombactZone`
  (if (not (`self.HasTriggerCinematic`))
    (set `self.HasTriggerCinematic` true)
    (bind _zonecombat (`self.ZoneCombat`)
      (:`then`
        (`/Game/Entities/NPCs/BP/Physics/BP_Zone.TriggerArena` _zonecombat self)
        (`self.K2_SetActorLocation` (`GameplayStatics.GetPlayerCharacter` 0) (`SceneComponent.K2_GetComponentLocation` (`/Game/Entities/NPCs/BP/Physics/BP_Zone.Sphere` _zonecombat)) false false)
        (`BlackboardComponent.SetValueAsBool` (`AIBlueprintHelperLibrary.GetBlackboard` null) (`self.StartEliteWait`) true))
      (:`else`))))

(event `self.AC_EnemyHealthSystem.OnDeath`
  (`/Game/Entities/NPCs/BP/Physics/BP_Zone.BreakArena` (`self.ZoneCombat`))
  (bind _asgm_base (cast `/Game/Core/GameModes/Game/GM_Base` (`GameplayStatics.GetGameMode`)))
  (set `/Game/Core/GameModes/Game/GM_Base.isInCombat` false _asgm_base))

(event `/Game/Entities/Player/BPI_IsEnemy.SetStunState`
  (params (Time :type "Float (double-precision)"))
  (bind _returnvalue (`AIBlueprintHelperLibrary.GetBlackboard` null))
  (`BlackboardComponent.SetValueAsBool` _returnvalue (`self.IsStun`) true)
  (`BlackboardComponent.SetValueAsFloat` _returnvalue (`self.Key Name`) Time))

(event `ChangeSkin`
  (set `SkeletalMeshComponent.SkeletalMeshAsset` "/Game/Entities/Character/Mesh/Elite/SK_ELITE.SK_ELITE" (`self.Mesh`)))

(fn `GotFound`
  (locals (AttackTarget :type Name :default "AttackTarget"))
  (`KismetSystemLibrary.PrintString` "Got you" true true (struct :`G` 0.66 :`B` 1.0 :`A` 1.0) 20.0)
  (`self.PlayAnimMontage` "/Game/Entities/NPCs/Enemies/Animations/Montages/AM_Attack2_Elite.AM_Attack2_Elite")
  (`BlackboardComponent.SetValueAsObject` (`AIBlueprintHelperLibrary.GetBlackboard` (`self.GetOwner`)) (`local.AttackTarget`) (`GameplayStatics.GetPlayerCharacter` 0)))

(fn `UserConstructionScript`)