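; Poolable enemy projectile wave that carries a group of bullets along a spline built from wave details.
; After a delayed start, it starts bullet lifetimes and a timeline advances the child actor by speed, rotating bullets to the spline.
; It tracks bullet deaths through bound events and signals DestroyWave when none remain or the path ends.
; Destroy resets movement, timer and bullet list for reuse instead of destroying the actor.
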(event `self.ReturnItem`
  (`parent.ReturnItem`)
  (`self.Destroy`)
  (clear `self.DestroyWave`))

(event `Move`
  (`Timeline|Chronologie` :!via `PlayFromStart` :!label _label
    (:`Update`
      (bind _done (`self.MoveChildActorAlongSpline` (`GameplayStatics.GetWorldDeltaSeconds`)))
      (if _done
        (`self.StopMove`)
        (`self.StopWave`)
        (elif (!= (`SplineComponent.GetNumberOfSplinePoints` (`self.Spline`)) 0)
          (`self.RotateBullet`))))))

(event `StopMove`
  (`KismetSystemLibrary.K2_ClearAndInvalidateTimerHandle` (`self.Timer`))
  (goto _label :!via `Stop`))

(event `StartMovingInTime`
  (params (TimeBeforeStart :type "Float (double-precision)"))
  (if (!= (`SplineComponent.GetNumberOfSplinePoints` (`self.Spline`)) 0)
    (for _ (`self.Bullets`)
      (`self.RotateBullet`)))
  (bind _returnvalue (`KismetSystemLibrary.K2_SetTimerDelegate` (delegate `StartMove`) (+ TimeBeforeStart 1.0)))
  (set `self.Timer` _returnvalue))

(event `StartMove`
  (`KismetSystemLibrary.K2_ClearAndInvalidateTimerHandle` (`self.Timer`))
  (bind _returnvalue (`KismetSystemLibrary.K2_SetTimerDelegate` (`|CreateDelegate` :!event `Move`) 1.0 true true))
  (set `self.Timer` _returnvalue)
  (for _array_element (`self.Bullets`)
    (set `/Game/Entities/NPCs/Enemies/BP/Character/BP_Projectile.Lifetime` (`.ProjectileLifetime_77_594EED6B4A51763397F473A18A51071B` (break `/Game/Data/Structs/S_WaveDetails` (`self.Details`))) _array_element)
    (`/Game/Entities/NPCs/Enemies/BP/Character/BP_Projectile.StartLifetime` _array_element))
  (`self.Move`))

(fn `AddBullet`
  (params (Bullet :type "/Game/Entities/NPCs/Enemies/BP/Character/BP_Projectile Object Reference"))
  (`KismetArrayLibrary.Array_Add` (`self.Bullets`) Bullet)
  (add `/Game/Entities/NPCs/Enemies/BP/Character/BP_Projectile.DestroyProjectile` (`local.Bullet`) (`|CreateDelegate` :!event `On Bullet Die`)))

(fn `BindEvent`
  (params (Bullet :type "/Game/Entities/NPCs/Enemies/BP/Character/BP_Projectile Object Reference"))
  (add `/Game/Entities/NPCs/Enemies/BP/Character/BP_Projectile.DestroyProjectile` Bullet (`|CreateDelegate` :!event `On Bullet Die`)))

(fn `Destroy`
  (`self.StopMove`)
  (`SceneComponent.K2_SetRelativeLocation` (`self.ChildActor`) (0.0 0.0 0.0) false false)
  (`KismetSystemLibrary.K2_ClearAndInvalidateTimerHandle` (`self.Timer`))
  (set `self.Speed` 0.0)
  (set `self.DistanceAlongSpline` 0.0)
  (`KismetArrayLibrary.Array_Clear` (`self.Bullets`))
  (return))

(fn `Init`
  (params (S_WaveDetails :type "/Game/Data/Structs/S_WaveDetails Structure"))
  (bind _output_get (set `self.Details` S_WaveDetails))
  (bind (_addeddelaybeforecast _delaybeforelaunch _attackpatterntype _splinepoints _tangents _direction _bullets _spawnonplayer _spawnoffset _projectilelifetime _projectilespeed) (break `/Game/Data/Structs/S_WaveDetails` _output_get))
  (set `self.Speed` _projectilespeed)
  (`self.SetSplinePoints` _splinepoints _tangents))

(fn `MoveChildActorAlongSpline`
  (params (DeltaTime :type "Float (double-precision)"))
  (returns (Done :type Boolean))
  (set `self.DistanceAlongSpline` (+ (* DeltaTime (`self.Speed`)) (`self.DistanceAlongSpline`)))
  (`SceneComponent.K2_SetRelativeLocation` (`self.ChildActor`) (`SplineComponent.GetLocationAtDistanceAlongSpline` (`self.Spline`) (`self.DistanceAlongSpline`) "Local") false false)
  (return (> (`self.DistanceAlongSpline`) (`SplineComponent.GetSplineLength` (`self.Spline`)))))

(fn `On Bullet Die`
  (params (Bullet :type "/Game/Entities/NPCs/Enemies/BP/Character/BP_Projectile Object Reference"))
  (`|ExecutionSequence`
    (:`then_1`
      (if (`KismetArrayLibrary.Array_Contains` (`self.Bullets`) Bullet)
        (`KismetArrayLibrary.Array_RemoveItem` (`self.Bullets`) (`local.Bullet`)))
      (if (`KismetArrayLibrary.Array_IsEmpty` (`self.Bullets`))
        (`self.DestroyWave` self)))))

(fn `RotateBullet`
  (for _array_element (`self.Bullets`)
    (`self.K2_SetActorRotation` _array_element (`SplineComponent.GetRotationAtDistanceAlongSpline` (`self.Spline`) (`self.DistanceAlongSpline`) "World") false)))

(fn `SetSplinePoints`
  (params (Points :type "Array of Vector Structure") (Tangents :type "Array of Vector Structure"))
  (`SplineComponent.ClearSplinePoints` (`self.Spline`) true)
  (for (_array_element _array_index) (`local.Points`)
    (`SplineComponent.AddPoint` (`self.Spline`) (make `SplinePoint` (`KismetMathLibrary.Conv_IntToDouble` _array_index) _array_element) false))
  (for (_array_element_2 _array_index_2) (`local.Tangents`)
    (`SplineComponent.SetTangentAtSplinePoint` (`self.Spline`) _array_index_2 _array_element_2 "Local" false))
  (`SplineComponent.UpdateSpline` (`self.Spline`)))

(fn `StopWave`
  (`self.StopMove`)
  (`KismetSystemLibrary.K2_ClearAndInvalidateTimerHandle` (`self.Timer`))
  (for _array_element (`self.Bullets`)
    (`|ExecutionSequence`
      (:`then_1`
        (`/Game/Entities/NPCs/Enemies/BP/Character/BP_Projectile.DestroyBullet` _array_element)
        (remove `/Game/Entities/NPCs/Enemies/BP/Character/BP_Projectile.DestroyProjectile` _array_element (`|CreateDelegate` :!event `On Bullet Die`)))))
  (`self.Destroy`)
  (`self.DestroyWave` self))

(fn `UserConstructionScript`)