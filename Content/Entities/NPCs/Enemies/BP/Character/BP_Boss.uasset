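; Boss enemy character that drives its AI controller through health-based phases and the end of the fight.
; Damage triggers phase 2 at half health, then phase 3 with damage disabled at minimal health; the next minimal-health hit ends the boss, gated by FlipFlop and DoN.
; ChangeHealth re-enables damage at one health point or disables it.
; DoDark fades screen-vision brightness through a timeline-driven Material Parameter Collection.
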(event `self.ReceiveBeginPlay`
  (bind _asaic_boss (cast `/Game/Entities/NPCs/Enemies/BP/AIController/AIC_Boss` (`self.GetController`)))
  (set `self.As AIC Boss` _asaic_boss)
  (add `/Game/Entities/Player/AC_EnemyHealthSystem.PlayerDamage` (`self.AC_EnemyHealthSystem`) (`|CreateDelegate` :!event `OnDamage`))
  (add `/Game/Entities/NPCs/Enemies/BP/Components/BPC_BossAttack.EndBoss` (`self.BPC_BossAttack`) (`|CreateDelegate` :!event `ChangeHealth`)))

(event `OnDamage`
  (bind _ac_enemyhealthsystem (`self.AC_EnemyHealthSystem`))
  (bind _currentheathpoints (`/Game/Entities/Player/AC_EnemyHealthSystem.currentHeathPoints` _ac_enemyhealthsystem))
  (if (<= _currentheathpoints 1.0)
    (`/Engine/EditorBlueprintResources/StandardMacros.FlipFlop`
      (:`A`
        (`/Engine/EditorBlueprintResources/StandardMacros.Do N` 1
          (:`Exit`
            (`/Game/Entities/NPCs/Enemies/BP/AIController/AIC_Boss.ChangePhase` (`self.As AIC Boss`) 3)
            (`/Game/Entities/Player/AC_EnemyHealthSystem.DeactivateDamage` (`self.AC_EnemyHealthSystem`)))))
      (:`B`
        (`/Engine/EditorBlueprintResources/StandardMacros.Do N` 1
          (:`Exit`
            (`/Game/Entities/NPCs/Enemies/BP/AIController/AIC_Boss.EndBoss` (`self.As AIC Boss`))))))
    (elif (<= (/ _currentheathpoints (`/Game/Entities/Player/AC_EnemyHealthSystem.maxHeathPoints` _ac_enemyhealthsystem)) 0.5)
      (`/Engine/EditorBlueprintResources/StandardMacros.Do N` 1
        (:`Exit`
          (`/Game/Entities/NPCs/Enemies/BP/AIController/AIC_Boss.ChangePhase` (`self.As AIC Boss`) 2))))))

(event `/Game/Entities/NPCs/Enemies/BP/Components/BPI_UseDark.DoDark`
  (params (GoDark :type Boolean))
  (`|ExecutionSequence`
    (:`then_0`
      (bind (_direction _newtrack_0) (`Timeline|Timeline` :`NewTime` 0.01 :!via `Stop` :!label _label)
        (:`Update`
          (`KismetMaterialLibrary.SetScalarParameterValue` "/Game/FX/EnemyFinder/MPC_Vision.MPC_Vision" "Brightness" _newtrack_0))))
    (:`then_1`
      (if GoDark
        (goto _label :!via `PlayFromStart`)
        (else
          (goto _label :!via `ReverseFromEnd`))))))

(event `ChangeHealth`
  (params (Val :type Boolean))
  (bind _ac_enemyhealthsystem (`self.AC_EnemyHealthSystem`))
  (if Val
    (`/Game/Entities/Player/AC_EnemyHealthSystem.ActivateDamage` _ac_enemyhealthsystem)
    (set `/Game/Entities/Player/AC_EnemyHealthSystem.currentHeathPoints` 1.0 _ac_enemyhealthsystem)
    (else
      (`/Game/Entities/Player/AC_EnemyHealthSystem.DeactivateDamage` (`self.AC_EnemyHealthSystem`)))))

(fn `UserConstructionScript`)