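; BP_PopCorn is an enemy NPC character Blueprint.
; On BeginPlay it passes its PopCornDetails actions to the attack component, which builds a cooldown table from them.
; SetStunState writes a stun flag and a time to the Blackboard for the AI.
; FireAnim toggles auto-activation on the claw slash Niagara effect, turning it off again after a fixed delay.
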(event `Fire Anim`
  (`ActorComponent.SetAutoActivate` (`self.NS_Enemies_Claw_Slash`) true)
  (`KismetSystemLibrary.Delay` 8.0)
  (`ActorComponent.SetAutoActivate` (`self.NS_Enemies_Claw_Slash`) false))

(event `self.ReceiveBeginPlay`
  (set `/Game/Entities/NPCs/Enemies/BP/Components/BPC_EnemyAttack.Actions` (`/Game/Data/DataAsset/PDA_EnemyAi.Actions` (`self.PopCornDetails`)) (`self.BPC_PopCornAttack`))
  (`/Game/Entities/NPCs/Enemies/BP/Components/BPC_EnemyAttack.CreateCooldownTable` (`self.BPC_PopCornAttack`)))

(event `/Game/Entities/Player/BPI_IsEnemy.SetStunState`
  (params (Time :type "Float (double-precision)"))
  (bind _returnvalue (`AIBlueprintHelperLibrary.GetBlackboard` null))
  (`BlackboardComponent.SetValueAsBool` _returnvalue (`self.IsStun`) true)
  (`BlackboardComponent.SetValueAsFloat` _returnvalue (`self.Key Name`) Time))

(fn `UserConstructionScript`)