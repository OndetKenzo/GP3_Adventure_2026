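; BP_Projectile is a pooled enemy projectile using the popcorn skeleton, with timed area attacks and a parry response that damages it.
; StartLifetime sets expiry and optional looping timers, while Attack triggers a capsule hit through the enemy combat system with Niagara effects.
; Expiry or leaving ArenaBound starts a delayed destroy notification, and ReturnItem resets hit state for reuse.
; Animation runs through Animation Sharing, driven by CrowdState.
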(event `self.ReceiveBeginPlay`
  (bind _returnvalue (`AnimationSharingManager.GetAnimationSharingManager`))
  (`AnimationSharingManager.RegisterActorWithSkeletonBP` _returnvalue self "/Game/Entities/Character/Mesh/Popcorn/SK_Popcorn_Skeleton.SK_Popcorn_Skeleton")
  (set `/Game/Entities/Player/AC_EnemyCombatSystem.characterMesh` (`self.SkeletalMesh`) (`self.AC_EnemyCombatSystem`))
  (set `self.Array` (`|MakeArray` "ObjectTypeQuery3" :!type "EObjectTypeQuery Enum")))

(event `RegisterAnim`
  (params (Anim :type "/Game/Entities/NPCs/Crowd/AnimationSharing/E_CrowdState Enum" :default "NewEnumerator0"))
  (set `self.CrowdState` Anim))

(event `self.GetItem`
  (`parent.GetItem`)
  (set `self.IsDestroying` false))

(event `self.ReturnItem`
  (`parent.ReturnItem`)
  (`self.K2_SetActorTransform` (`KismetMathLibrary.MakeTransform` (0.0 0.0 0.0)) false true)
  (clear `self.DestroyProjectile`)
  (`/Game/Entities/Player/AC_EnemyCombatSystem.ClearHitActors` (`self.AC_EnemyCombatSystem`))
  (set `self.CrowdState` "NewEnumerator0"))

(event `StartLifetime`
  (bind _attackdelay (`self.AttackDelay`))
  (`KismetSystemLibrary.K2_ClearAndInvalidateTimerHandle` (`self.Timer`))
  (bind _returnvalue (`KismetSystemLibrary.K2_SetTimerDelegate` (delegate `DestroyBullet`) (`self.Lifetime`) false true))
  (set `self.Timer` _returnvalue)
  (if (not (< _attackdelay 0.0))
    (if (== _attackdelay 0.0)
      (set `self.AttackDelay` 0.1))
    (bind _returnvalue_2 (`KismetSystemLibrary.K2_SetTimerDelegate` (`|CreateDelegate` :!event `Attack`) (`self.AttackDelay`) true true))
    (set `self.AttackTimer` _returnvalue_2)))

(event `DestroyBullet`
  (`self.IsDestroying`
    (:`then`)
    (:`else`
      (set `self.IsDestroying` true)
      (`ActorComponent.Deactivate` (`self.Niagara1`))
      (`ActorComponent.Deactivate` (`self.Niagara`))
      (`ActorComponent.Deactivate` (`self.Niagara2`))
      (`KismetSystemLibrary.K2_ClearAndInvalidateTimerHandle` (`self.Timer`))
      (`KismetSystemLibrary.K2_ClearAndInvalidateTimerHandle` (`self.AttackTimer`))
      (`self.K2_DetachFromActor` "KeepWorld" "KeepWorld" "KeepWorld")
      (set `self.CrowdState` "NewEnumerator13")
      (set `self.IsDestroying` true)
      (`KismetSystemLibrary.K2_SetTimerDelegate` (delegate `CustomEvent`) 1.0))))

(event `CustomEvent`
  (`KismetSystemLibrary.K2_ClearAndInvalidateTimerHandle` (`self.Timer`))
  (`self.DestroyProjectile` self)
  (clear `self.DestroyProjectile`))

(event `self.Capsule.OnComponentEndOverlap`
  (params (OverlappedComponent :type "PrimitiveComponent Object Reference") (OtherActor :type "Actor Object Reference") (OtherComp :type "PrimitiveComponent Object Reference") (OtherBodyIndex :type Integer))
  (if (`self.ActorHasTag` OtherActor "ArenaBound")
    (`self.DestroyBullet`)))

(event `Attack`
  (`/Game/Entities/Player/AC_EnemyCombatSystem.Trigger HitCapsule` (`self.AC_EnemyCombatSystem`) (`self.AttackDamage`) (`self.AttackRadius`) (`self.Array`) (`self.K2_GetActorLocation`))
  (if (> (`self.AttackDelay`) 0.1)
    (set `self.CrowdState` "NewEnumerator11")
    (`ActorComponent.Activate` (`self.Niagara`) true)
    (else
      (set `self.CrowdState` "NewEnumerator12")
      (`ActorComponent.Activate` (`self.Niagara1`) false))))

(event `/Game/Entities/Player/PlayerCombatSystem/BPI_RespondParry.RespondToParry`
  (params (Parrier :type "Actor Object Reference"))
  (`/Game/Entities/Player/AC_EnemyHealthSystem.OnTakePointDamage_Event` (`self.AC_EnemyHealthSystem`) null 1.0 null (`self.K2_GetActorLocation` Parrier) null "None" (0.0 0.0 0.0) null Parrier))

(event `PlaySfx`)

(fn `GetCrowdState`
  (params (OnDemandeState :type Byte) (CurrentState :type Byte))
  (returns (State :type "/Game/Entities/NPCs/Crowd/AnimationSharing/E_CrowdState Enum"))
  (if (!= OnDemandeState 255)
    (`self.IsOnDemand`
      (:`then`
        _)
      (:`else`
        (set `self.IsOnDemand` true)))
    (return (`self.CrowdState`))
    (elif (`self.IsOnDemand`)
      (set `self.IsOnDemand` false)
      (bind _output_get (set `self.CrowdState` (cast `/Game/Entities/NPCs/Crowd/AnimationSharing/E_CrowdState` (`local.CurrentState`))))
      (return _output_get)
      (else
        (return (`self.CrowdState`))))))

(fn `UserConstructionScript`)