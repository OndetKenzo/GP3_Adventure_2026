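; Enemy NPC component that teleports its owner to a random actor tagged "Teleport", excluding the point closest to the owner.
; Points are gathered shortly after BeginPlay; the move copies the chosen point's location and yaw.
; TeleportToRandomPoint either moves immediately or uses timed stages, playing the AM_TP montage in reverse before the move and forward after it.
; A callback is invoked after each teleport.
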(event `self.ReceiveBeginPlay`
  (`KismetSystemLibrary.Delay` 2.0)
  (bind _outactors (`GameplayStatics.GetAllActorsWithTag` "Teleport"))
  (set `self.Points` _outactors))

(event `TeleportToRandomPoint`
  (params (DoAnim :type Boolean))
  (if DoAnim
    (bind _returnvalue (`KismetSystemLibrary.K2_SetTimerDelegate` (`|CreateDelegate` :!event `Tp1`) (`self.TimeTpUp`)))
    (set `self.Timer` _returnvalue)
    (else
      (`self.Teleport`)
      (`self.CallBack`))))

(event `Tp1`
  (`KismetSystemLibrary.K2_ClearAndInvalidateTimerHandle` (`self.Timer`))
  (`KismetSystemLibrary.K2_SetTimerDelegate` (`|CreateDelegate` :!event `Tp2`) (`self.TimeTpDown`))
  (`|PlayMontage` (`Actor.GetComponentByClass` (`self.GetOwner`) "/Script/Engine.SkeletalMeshComponent") "/Game/Entities/Character/Mesh/Antagonist/Animations/AM_TP.AM_TP" -1.0 2.237))

(event `Tp2`
  (`KismetSystemLibrary.K2_ClearAndInvalidateTimerHandle` (`self.Timer`))
  (`self.Teleport`)
  (`self.CallBack`)
  (`|PlayMontage` (`Actor.GetComponentByClass` (`self.GetOwner`) "/Script/Engine.SkeletalMeshComponent") "/Game/Entities/Character/Mesh/Antagonist/Animations/AM_TP.AM_TP"))

(fn `BPC_TeleportComponent_AutoGenFunc`)

(fn `GetClosest`
  (returns (Actor :type "Actor Object Reference"))
  (locals (Closest :type "Actor Object Reference") (MinDist :type "Float (single-precision)" :default 0.0))
  (bind _points (`self.Points`))
  (bind _output (`|GetArrayItem` _points))
  (set `local.MinDist` (`Actor.GetDistanceTo` (`self.GetOwner`) _output))
  (set `local.Closest` _output)
  (for _array_element _points
    (bind _returnvalue (`Actor.GetDistanceTo` _array_element (`self.GetOwner`)))
    (if (< _returnvalue (`local.MinDist`))
      (set `local.Closest` _array_element)
      (set `local.MinDist` _returnvalue)))
  (return (`local.Closest`)))

(fn `Teleport`
  (locals (Actor :type "Actor Object Reference"))
  (bind _returnvalue (`Actor.GetTransform` (`local.Actor`)))
  (bind _actor (`self.GetClosest`))
  (set `local.Actor` (`KismetArrayLibrary.Array_Random` (`self.Points`)))
  (while (== _actor (`local.Actor`))
    (set `local.Actor` (`KismetArrayLibrary.Array_Random` (`self.Points`))))
  (`Actor.K2_SetActorTransform` (`self.GetOwner`) (`KismetMathLibrary.MakeTransform` (.location _returnvalue) (`KismetMathLibrary.MakeRotator` 0.0 0.0 (.yaw (.rotation _returnvalue)))) false false))