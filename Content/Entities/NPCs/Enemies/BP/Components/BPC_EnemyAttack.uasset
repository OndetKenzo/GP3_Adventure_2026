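; Enemy attack component that runs named actions from a map for NPC enemies and tracks a cooldown for each.
; A looping timer counts cooldowns down to zero, and executing an action resets its cooldown and async-loads its montage.
; It spawns an orange or red halo test VFX for blockable or unblockable attacks, snaps the owner toward the player, and plays the montage.
; Start and finish events notify listeners, including on interruption or a missing action.
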(event `CreateCooldownTable`
  (`BlueprintMapLibrary.Map_Clear` (`self.ActionCooldowns`))
  (bind _keypin (`|MapForEach` (`self.Actions`))
    (:`then`
      (`BlueprintMapLibrary.Map_Add` (`self.ActionCooldowns`) _keypin))))

(event `self.ReceiveBeginPlay`
  (set `self.Mesh` (`Actor.GetComponentByClass` (`self.GetOwner`) "/Script/Engine.SkeletalMeshComponent"))
  (`KismetSystemLibrary.K2_SetTimerDelegate` (delegate `UpdateCooldowns`) (`self.CooldownRefreshRate`) true))

(event `UpdateCooldowns`
  (bind (_keypin _valuepin) (`|MapForEach` (`self.ActionCooldowns`))
    (:`then`
      (`BlueprintMapLibrary.Map_Add` (`self.ActionCooldowns`) _keypin (`KismetMathLibrary.FMax` (- _valuepin (`self.CooldownRefreshRate`)))))))

(event `ExecuteAction`
  (params (Action :type "/Game/Data/Enum/E_Actions Enum" :default "NewEnumerator0"))
  (bind _mesh (`self.Mesh`))
  (bind (_value _returnvalue) (`BlueprintMapLibrary.Map_Find` (`self.Actions`) Action))
  (bind (_priority _weight _montagetoplay _interruptable _parryable _blockable _cooldown) (break `/Game/Data/Structs/S_ActionDetails` _value))
  (`self.OnActionStarted`)
  (if _returnvalue
    (`BlueprintMapLibrary.Map_Add` (`self.ActionCooldowns`) Action _cooldown)
    (bind _object (`|LoadAsset` _montagetoplay)
      (:`Completed`
        (bind _asanim_montage (cast `AnimMontage` _object))
        (if _blockable
          (`NiagaraFunctionLibrary.SpawnSystemAttached` "/Game/FX/Enemies/Halo/NS_Attack_Halo_Orange.NS_Attack_Halo_Orange" _mesh "None" (0.0 0.0 100.0) (struct) "SnapToTarget" true)
          (else
            ; Test VFX
            (`NiagaraFunctionLibrary.SpawnSystemAttached` "/Game/FX/Enemies/Halo/NS_Attack_Halo_Red.NS_Attack_Halo_Red" _mesh "None" (0.0 0.0 100.0) (struct) "SnapToTarget" true)))
        (`Actor.K2_SetActorRotation` (`self.GetOwner`) (`KismetMathLibrary.FindLookAtRotation` (`Actor.K2_GetActorLocation` (`self.GetOwner`)) (`Actor.K2_GetActorLocation` (`GameplayStatics.GetPlayerCharacter` 0))) false)
        (`|PlayMontage` _mesh _asanim_montage 1.8
          (:`OnCompleted`
            _)
          (:`OnInterrupted`
            _))
        (`self.OnActionFinished`)))
    (else
      (`KismetSystemLibrary.PrintText` "No Action Found")
      (`self.OnActionFinished`))))