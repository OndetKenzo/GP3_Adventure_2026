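; BP_NpcManager is a test manager that shows and hides a batch of pooled actors, presumably NPCs, through a trigger box or the H key.
; Box overlap or pressing H pulls 100 actors from ActorPool once, guarded by IsSpawned, and places them at incremental offsets from the box.
; End overlap or releasing H pushes them back to the pool and resets the state.
; Overlaps are not filtered by actor.
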(event `self.Box.OnComponentBeginOverlap`
  (params (OverlappedComponent :type "PrimitiveComponent Object Reference") (OtherActor :type "Actor Object Reference") (OtherComp :type "PrimitiveComponent Object Reference") (OtherBodyIndex :type Integer) (bFromSweep :type Boolean) (SweepResult :type "HitResult Structure (by ref)"))
  (if (not (`self.IsSpawned`)) :!label _label
    (set `self.IsSpawned` true)
    (`KismetSystemLibrary.PrintString` "Appear")
    (for _ (range 100)
      (bind _returnvalue (`ActorPoolComponent.Pull` (`self.ActorPool`)))
      (`KismetArrayLibrary.Array_Add` (`self.SpawnedActors`) _returnvalue)
      (`self.K2_SetActorLocation` _returnvalue (+ (`SceneComponent.K2_GetComponentLocation` (`self.Box`)) (* (`self.Offset`) (`KismetMathLibrary.Conv_IntToVector` (`self.iteration`)))) false false)
      (set `self.iteration` (+ (`self.iteration`) 1)))))

(event `Key|H`
  (params (Key :type "Key Structure"))
  (bind _spawnedactors (`self.SpawnedActors`))
  (:`Pressed`
    (goto _label))
  (:`Released`
    (`KismetSystemLibrary.PrintString` "Disappear" :!label _label_2)
    (set `self.IsSpawned` false)
    (for _array_element _spawnedactors
      (`ActorPoolComponent.Push` (`self.ActorPool`) _array_element))
    (`KismetArrayLibrary.Array_Clear` _spawnedactors)
    (set `self.iteration` 0)))

(event `self.Box.OnComponentEndOverlap`
  (params (OverlappedComponent :type "PrimitiveComponent Object Reference") (OtherActor :type "Actor Object Reference") (OtherComp :type "PrimitiveComponent Object Reference") (OtherBodyIndex :type Integer))
  (goto _label_2))

(fn `UserConstructionScript`)