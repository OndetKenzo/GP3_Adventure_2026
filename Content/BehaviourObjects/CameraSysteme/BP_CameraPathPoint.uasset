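; Camera path point actor that previews a camera placement in the editor; it has no runtime logic.
; The construction script clears persistent debug lines, then computes four frustum corners from the actor location plus CameraOffset, using CameraRotation for direction and CameraFov as the half-extent at a fixed distance.
; It draws the resulting pyramid with long-lived debug arrows and marks the origin with a debug sphere.
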(fn `UserConstructionScript`
  (locals (UpLeft :type "Vector Structure") (UpRight :type "Vector Structure") (Origine :type "Vector Structure") (DownRight :type "Vector Structure") (DownLeft :type "Vector Structure"))
  (bind (_camerarotation_x _camerarotation_y) (`KismetMathLibrary.BreakVector2D` (`self.CameraRotation`)))
  (bind _returnvalue (`KismetMathLibrary.MakeRotator` 0.0 _camerarotation_x _camerarotation_y))
  (bind _returnvalue_2 (* (`KismetMathLibrary.GetUpVector` _returnvalue) (`self.CameraFov`)))
  (bind _returnvalue_3 (* (`KismetMathLibrary.GetRightVector` _returnvalue) (`self.CameraFov`)))
  (bind _returnvalue_4 (* (`KismetMathLibrary.GetForwardVector` _returnvalue) 200.0))
  (bind _returnvalue_5 (+ _returnvalue_4 _returnvalue_3))
  (bind _returnvalue_6 (- _returnvalue_4 _returnvalue_3))
  (`KismetSystemLibrary.FlushPersistentDebugLines`)
  (set `local.Origine` (+ (`self.K2_GetActorLocation`) (`self.CameraOffset`)))
  (set `local.UpRight` (+ (+ _returnvalue_5 _returnvalue_2) (`local.Origine`)))
  (set `local.UpLeft` (+ (+ _returnvalue_6 _returnvalue_2) (`local.Origine`)))
  (set `local.DownRight` (+ (- _returnvalue_5 _returnvalue_2) (`local.Origine`)))
  (set `local.DownLeft` (+ (- _returnvalue_6 _returnvalue_2) (`local.Origine`)))
  (`KismetSystemLibrary.DrawDebugArrow` (`local.Origine`) (`local.UpLeft`) 1.0 (struct :`B` 1.0 :`A` 1.0) 2000.0 1.0)
  (`KismetSystemLibrary.DrawDebugArrow` (`local.Origine`) (`local.UpRight`) 1.0 (struct :`B` 1.0 :`A` 1.0) 2000.0 1.0)
  (`KismetSystemLibrary.DrawDebugArrow` (`local.Origine`) (`local.DownLeft`) 1.0 (struct :`B` 1.0 :`A` 1.0) 2000.0 1.0)
  (`KismetSystemLibrary.DrawDebugArrow` (`local.Origine`) (`local.DownRight`) 1.0 (struct :`B` 1.0 :`A` 1.0) 2000.0 1.0)
  (`KismetSystemLibrary.DrawDebugArrow` (`local.UpLeft`) (`local.UpRight`) 1.0 (struct :`B` 1.0 :`A` 1.0) 2000.0 1.0)
  (`KismetSystemLibrary.DrawDebugArrow` (`local.UpRight`) (`local.DownRight`) 1.0 (struct :`B` 1.0 :`A` 1.0) 2000.0 1.0)
  (`KismetSystemLibrary.DrawDebugArrow` (`local.DownRight`) (`local.DownLeft`) 1.0 (struct :`B` 1.0 :`A` 1.0) 2000.0 1.0)
  (`KismetSystemLibrary.DrawDebugArrow` (`local.DownLeft`) (`local.UpLeft`) 1.0 (struct :`B` 1.0 :`A` 1.0) 2000.0 1.0)
  (`KismetSystemLibrary.DrawDebugSphere` (`local.Origine`) 25.0 12 (struct :`R` 1.0 :`G` 1.0 :`B` 1.0 :`A` 1.0) 2000.0))