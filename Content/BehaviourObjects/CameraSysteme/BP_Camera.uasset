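; Game camera actor that becomes the player's view target and switches between Platform, Search, Exploration and Fight states.
; Search, Exploration and Fight ease to a player-relative offset at set angles.
; Platform finds the player's nearest BP_CameraPath spline key and blends adjacent points' offset, rotation or look-at, and FOV.
; Path events toggle Platform, checkpoints restore state, and MPC_Player receives player position and transparency for a see-through shader.
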(event `self.ReceiveBeginPlay`
  ;[0.1912 0.1912 0.8781 0.5] BeginPlay
  ;; Get Player If none selected
  (`KismetSystemLibrary.DelayUntilNextTick`)
  (`self.SetCamToPlayer`)
  ;; Connect to all Path
  (bind _outactors (`GameplayStatics.GetAllActorsOfClass` "/Game/BehaviourObjects/CameraSysteme/BP_CameraPath.BP_CameraPath_C"))
  (for _array_element _outactors
    (add `/Game/BehaviourObjects/CameraSysteme/BP_CameraPath.OnPlayerEnteredPath` _array_element (`|CreateDelegate` :!event `HandlePathEntered`))))

(event `self.ReceiveTick`
  (params (DeltaSeconds :type "Float (single-precision)"))
  ;[0.5617 0.5409 0.15 0.5] Tick
  (`|ExecutionSequence`
    (:`then_0`
      ;; GivePlayerPosToSeeThroughShader
      (`/Engine/EditorBlueprintResources/StandardMacros.IsValid` (`self.Player`)
        (:`Is Valid`
          (`KismetMaterialLibrary.SetVectorParameterValue` "/Game/Shaders/See_Through/MPC_Player.MPC_Player" "PlayerPos" (`KismetMathLibrary.Conv_VectorToLinearColor` (`self.K2_GetActorLocation` (`self.Player`)))))))
    (:`then_1`
      ;; HandleStates
      (switch `/Game/BehaviourObjects/CameraSysteme/EN_CameraStates` (`self.CameraState`)
        (:`NewEnumerator0`
          (`self.Platform`))
        (:`NewEnumerator1`
          (`self.Search`))
        (:`NewEnumerator2`
          (`self.Exploration`))
        (:`NewEnumerator3`
          (`self.Fight`))))))

(event `HandlePathEntered`
  (params (CameraPath :type "/Game/BehaviourObjects/CameraSysteme/BP_CameraPath Object Reference") (IsExitOne :type Boolean))
  (bind _actualspline (`self.ActualSpline`))
  ;[0.6823 0.1144 0.1144 0.5] Handle Plateform Enter/Exit
  (if (== (enumliteral `/Game/BehaviourObjects/CameraSysteme/EN_CameraStates` "NewEnumerator0") (`KismetSystemLibrary.MakeLiteralByte` (`self.CameraState`)))
    ;; Set Exploration State
    (set `self.CameraState` (enumliteral `/Game/BehaviourObjects/CameraSysteme/EN_CameraStates` "NewEnumerator2"))
    ;;; Reset Camera Rotation and Fov By exit
    (set `self.RotationPlayerExploration` (`KismetMathLibrary.SelectFloat` (`/Game/BehaviourObjects/CameraSysteme/BP_CameraPath.AngleExit1` _actualspline) (`/Game/BehaviourObjects/CameraSysteme/BP_CameraPath.AngleExit2` _actualspline) IsExitOne))
    (`CameraComponent.SetFieldOfView` (`self.Camera`) (`KismetMathLibrary.SelectFloat` (`/Game/BehaviourObjects/CameraSysteme/BP_CameraPath.ExitFov` _actualspline) (`/Game/BehaviourObjects/CameraSysteme/BP_CameraPath.ExitFov2` _actualspline) IsExitOne))
    (else
      ;; Set Platform State
      (set `self.CameraState` (enumliteral `/Game/BehaviourObjects/CameraSysteme/EN_CameraStates` "NewEnumerator0"))
      (set `self.ActualSpline` CameraPath))))

(event `SetCameraValueAtCheckPoint`
  (params (Checkpoint :type "/Game/Core/Optimisations/CheckpointSystem/BP_Checkpoint Object Reference"))
  (bind _camerastate (`/Game/Core/Optimisations/CheckpointSystem/BP_Checkpoint.CameraState` Checkpoint))
  (if (== (`KismetSystemLibrary.MakeLiteralByte` (`self.CameraState`)) _camerastate)
    (`KismetSystemLibrary.PrintString` "truemageule")
    (else
      (set `self.CameraState` _camerastate)
      (set `self.ActualSpline` (`/Game/Core/Optimisations/CheckpointSystem/BP_Checkpoint.ClosestCameraPath` Checkpoint)))))

(fn `Exploration`
  (bind _rotationplayerexploration (`self.RotationPlayerExploration`))
  (`self.SetPosition` (`self.DistPlayerExploration`) _rotationplayerexploration)
  (`self.K2_SetActorRotation` (`KismetMathLibrary.MakeRotator` 0.0 (`self.AnglePlayerExploration`) _rotationplayerexploration)))

(fn `Fight`
  (bind _rotationplayerexploration (`self.RotationPlayerExploration`))
  (`self.SetPosition` (`self.DistPlayerFight`) _rotationplayerexploration)
  (`self.K2_SetActorRotation` (`KismetMathLibrary.MakeRotator` 0.0 (`self.AnglePlayerExploration`) _rotationplayerexploration)))

(fn `LerpCamera`
  (params (Closest :type "/Game/BehaviourObjects/CameraSysteme/ST_CameraPoints Structure") (SecondClosest :type "/Game/BehaviourObjects/CameraSysteme/ST_CameraPoints Structure") (FirstPos :type "Vector Structure") (SecPos :type "Vector Structure") (Step :type "Float (double-precision)"))
  (`self.PlatformSetPosition` Closest SecondClosest FirstPos SecPos Step)
  (`self.PlaformSetRotation` Closest SecondClosest Step)
  (`self.PlatformSetFov` Closest SecondClosest Step)
  (`KismetMaterialLibrary.SetScalarParameterValue` "/Game/Shaders/See_Through/MPC_Player.MPC_Player" "UseTransparency" (`KismetMathLibrary.SelectFloat` (`KismetMathLibrary.SelectFloat` 1.0 0.0 (`.UseTransparency_31_71CB12874D6251A3C94DF9827C1E51A3` (break `/Game/BehaviourObjects/CameraSysteme/ST_CameraPoints` Closest))) (`KismetMathLibrary.SelectFloat` 1.0 0.0 (`.UseTransparency_31_71CB12874D6251A3C94DF9827C1E51A3` (break `/Game/BehaviourObjects/CameraSysteme/ST_CameraPoints` SecondClosest))) (< Step 0.5))))

(fn `PlaformSetRotation`
  (params (Closest :type "/Game/BehaviourObjects/CameraSysteme/ST_CameraPoints Structure") (SecondClosest :type "/Game/BehaviourObjects/CameraSysteme/ST_CameraPoints Structure") (step :type "Float (double-precision)"))
  (bind (_camerarotation _cameraoffset _camerafov _camerafix) (break `/Game/BehaviourObjects/CameraSysteme/ST_CameraPoints` SecondClosest))
  (bind (_camerarotation_2 _cameraoffset_2 _camerafov_2 _camerafix_2) (break `/Game/BehaviourObjects/CameraSysteme/ST_CameraPoints` Closest))
  ; Get Spline Point Rotation And If Need To Look at this Rotation
  (if (< step 0.5)
    (if _camerafix_2
      ; Lerp To The Look Rotation Of The Spline
      (`self.K2_SetActorRotation` (`KismetMathLibrary.RInterpTo` (`self.K2_GetActorRotation`) (`KismetMathLibrary.RLerp` (`KismetMathLibrary.MakeRotator` 0.0 (+ (`KismetMathLibrary.BreakVector2D` _camerarotation_2) 90.0) (`.Y` (`KismetMathLibrary.BreakVector2D` _camerarotation_2))) (`KismetMathLibrary.MakeRotator` 0.0 (+ (`KismetMathLibrary.BreakVector2D` _camerarotation) 90.0) (`.Y` (`KismetMathLibrary.BreakVector2D` _camerarotation))) step) (`GameplayStatics.GetWorldDeltaSeconds`) 1.0) :!label _label)
      (else
        ; Look At The Player
        (`self.K2_SetActorRotation` (`KismetMathLibrary.RInterpTo` (`self.K2_GetActorRotation`) (`KismetMathLibrary.MakeRotator` 0.0 (+ (.pitch (`KismetMathLibrary.FindLookAtRotation` (`self.K2_GetActorLocation`) (`self.K2_GetActorLocation` (`self.Player`)))) 90.0) (.yaw (`KismetMathLibrary.FindLookAtRotation` (`self.K2_GetActorLocation`) (`self.K2_GetActorLocation` (`self.Player`))))) (`GameplayStatics.GetWorldDeltaSeconds`) 1.0) :!label _label_2)))
    (elif _camerafix
      (goto _label)
      (else
        (goto _label_2))))
  (return))

(fn `Platform`
  (`/Engine/EditorBlueprintResources/StandardMacros.IsValid` (`self.ActualSpline`)
    (:`Is Valid`
      (bind (_closest _secondclosest _firstpos _secpos _step) (`self.SetPointsValue`))
      (`self.LerpCamera` _closest _secondclosest _firstpos _secpos _step))
    (:`Is Not Valid`
      (set `self.CameraState` "NewEnumerator2"))))

(fn `PlatformSetFov`
  (params (Closest :type "/Game/BehaviourObjects/CameraSysteme/ST_CameraPoints Structure") (SecondClosest :type "/Game/BehaviourObjects/CameraSysteme/ST_CameraPoints Structure") (Step :type "Float (double-precision)"))
  (bind (_camerarotation _cameraoffset _camerafov _camerafix _usefov) (break `/Game/BehaviourObjects/CameraSysteme/ST_CameraPoints` Closest))
  (bind (_camerarotation_2 _cameraoffset_2 _camerafov_2 _camerafix_2 _usefov_2) (break `/Game/BehaviourObjects/CameraSysteme/ST_CameraPoints` SecondClosest))
  (bind _camera (`self.Camera`))
  (bind _camera_2 (`self.Camera`))
  ; Check If Fov Needed
  (if (< Step 0.5)
    (if _usefov
      ; Lerp To the Spline Point Fov
      (`CameraComponent.SetFieldOfView` _camera (`KismetMathLibrary.FInterpTo` (`CameraComponent.FieldOfView` _camera) (`KismetMathLibrary.Lerp` _camerafov _camerafov_2 Step) (`GameplayStatics.GetWorldDeltaSeconds`) 1.0) :!label _label)
      (else
        ; Lerp To the Base Fov
        (`CameraComponent.SetFieldOfView` _camera_2 (`KismetMathLibrary.FInterpTo` (`CameraComponent.FieldOfView` _camera_2) (`self.BaseFov`) (`GameplayStatics.GetWorldDeltaSeconds`) 1.0) :!label _label_2)))
    (elif _usefov_2
      (goto _label)
      (else
        (goto _label_2)))))

(fn `PlatformSetPosition`
  (params (Closest :type "/Game/BehaviourObjects/CameraSysteme/ST_CameraPoints Structure") (SecondClosest :type "/Game/BehaviourObjects/CameraSysteme/ST_CameraPoints Structure") (FirstPos :type "Vector Structure") (SecPos :type "Vector Structure") (Step :type "Float (double-precision)"))
  (`self.K2_SetActorLocation` (`KismetMathLibrary.VInterpTo` (`self.K2_GetActorLocation`) (`KismetMathLibrary.VLerp` (+ (`.CameraOffset_27_0099F0B2440FEB464C0730A823FA62B1` (break `/Game/BehaviourObjects/CameraSysteme/ST_CameraPoints` Closest)) FirstPos) (+ (`.CameraOffset_27_0099F0B2440FEB464C0730A823FA62B1` (break `/Game/BehaviourObjects/CameraSysteme/ST_CameraPoints` SecondClosest)) SecPos) Step) (`GameplayStatics.GetWorldDeltaSeconds`) 2.0))
  (return))

(fn `Search`
  (bind _rotationplayersearch (`self.RotationPlayerSearch`))
  (`self.SetPosition` (`self.DistPlayerSearch`) _rotationplayersearch)
  (`self.K2_SetActorRotation` (`KismetMathLibrary.MakeRotator` 0.0 (`self.AnglePlayerExploration`) _rotationplayersearch)))

(fn `SetCamToPlayer`
  ; Check Player Valid
  (`/Engine/EditorBlueprintResources/StandardMacros.IsValid` (`self.Player`)
    (:`Is Not Valid`
      ; Set Player
      (bind _asbp_player (cast `/Game/Entities/Player/BP_Player` (`GameplayStatics.GetPlayerCharacter` 0)))
      (set `self.Player` _asbp_player)
      (`PlayerController.SetViewTargetWithBlend` (`GameplayStatics.GetPlayerController` 0) self 0.0 "VTBlend_Linear" 0.0 false)
      (return))))

(fn `SetPointsValue`
  (returns (Closest :type "/Game/BehaviourObjects/CameraSysteme/ST_CameraPoints Structure") (SecondClosest :type "/Game/BehaviourObjects/CameraSysteme/ST_CameraPoints Structure") (FirstPos :type "Vector Structure") (SecPos :type "Vector Structure") (Step :type "Float (double-precision)"))
  (locals (ClosestPoint :type "/Game/BehaviourObjects/CameraSysteme/BP_CameraPathPoint Object Reference") (SecondCloses :type "/Game/BehaviourObjects/CameraSysteme/BP_CameraPathPoint Object Reference") (ClosestIndex :type Integer) (PlayerLoc :type "Vector Structure" :default (0.0 0.0 0.0)))
  (bind _actualspline (`self.ActualSpline`))
  (bind _arraypoints (`/Game/BehaviourObjects/CameraSysteme/BP_CameraPath.ArrayPoints` (`self.ActualSpline`)))
  (bind _spline (`/Game/BehaviourObjects/CameraSysteme/BP_CameraPath.Spline` (`self.ActualSpline`)))
  (bind _returnvalue (`SplineComponent.FindInputKeyClosestToWorldLocation` (`/Game/BehaviourObjects/CameraSysteme/BP_CameraPath.Spline` (`self.ActualSpline`)) (`self.K2_GetActorLocation` (`self.Player`))))
  (bind _returnvalue_2 (`KismetMathLibrary.FFloor` _returnvalue))
  (bind _returnvalue_3 (`KismetMathLibrary.FCeil` _returnvalue))
  (bind _returnvalue_4 (- (`SceneComponent.K2_GetComponentLocation` (`/Game/BehaviourObjects/CameraSysteme/BP_CameraPath.Spline` _actualspline)) (`self.K2_GetActorLocation` _actualspline)))
  (return (`|GetArrayItem` _arraypoints _returnvalue_2) (`|GetArrayItem` _arraypoints _returnvalue_3) (- (`SplineComponent.GetLocationAtSplinePoint` _spline _returnvalue_2 "World") _returnvalue_4) (- (`SplineComponent.GetLocationAtSplinePoint` _spline _returnvalue_3 "World") _returnvalue_4) (`KismetMathLibrary.Fraction` _returnvalue)))

(fn `SetPosition`
  (params (DistPlayer :type "Vector2D Structure") (RotationPlayer :type "Float (double-precision)"))
  ; Camera Position Relative to the Player
  (bind _player (`self.Player`)
    (:`then`
      (bind (_returnvalue_x _returnvalue_y _returnvalue_z) (`KismetMathLibrary.BreakVector` (`self.K2_GetActorLocation` _player)))
      (`self.K2_SetActorLocation` (`KismetMathLibrary.VInterpTo` (`self.K2_GetActorLocation`) (`KismetMathLibrary.MakeVector` (+ _returnvalue_x (* DistPlayer_X (`KismetMathLibrary.DegCos` RotationPlayer))) (+ (* (`KismetMathLibrary.DegSin` RotationPlayer) DistPlayer_X) _returnvalue_y) (+ _returnvalue_z (* DistPlayer_Y -1.0))) (`GameplayStatics.GetWorldDeltaSeconds`) 1.0)))
    (:`else`)))

(fn `TestFunc`
  (returns (ReturnValue :type "Float (double-precision)"))
  (bind _camerapathpoint (`self.CameraPathPoint`))
  (bind _returnvalue (`self.K2_GetActorLocation` _camerapathpoint))
  (bind _returnvalue_2 (- (`self.K2_GetActorLocation` (`/Game/BehaviourObjects/CameraSysteme/BP_CameraPathPoint.NextPoint` _camerapathpoint)) _returnvalue))
  (return (/ (`KismetMathLibrary.Dot_VectorVector` (- (`self.K2_GetActorLocation` (`self.Player`)) _returnvalue) _returnvalue_2) (`KismetMathLibrary.Dot_VectorVector` _returnvalue_2 _returnvalue_2))))

(fn `UserConstructionScript`)