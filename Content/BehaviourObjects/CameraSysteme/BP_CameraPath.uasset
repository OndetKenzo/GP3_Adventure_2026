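; BP_CameraPath is a spline-based camera path that notifies BP_Camera actors when the player enters it.
; At BeginPlay it binds its OnPlayerEnteredPath dispatcher for each camera, then on player overlap broadcasts itself and whether EntryExit1 is the nearer end.
; The construction script draws debug frustums from each ArrayPoints entry's offset, rotation and FOV at its spline point.
; Logic to rebuild ArrayPoints from the spline is present but disconnected.
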(event `self.ReceiveBeginPlay`
  (bind _outactors (`GameplayStatics.GetAllActorsOfClass` "/Game/BehaviourObjects/CameraSysteme/BP_Camera.BP_Camera_C"))
  (for _array_element _outactors
    (add `self.OnPlayerEnteredPath` (`|CreateDelegate` _array_element :!event `HandlePathEntered`))))

(event `self.ReceiveActorBeginOverlap`
  (params (OtherActor :type "Actor Object Reference"))
  (bind _returnvalue (`self.K2_GetActorLocation` OtherActor))
  (set `self.IsExitOne` (< (`KismetMathLibrary.Vector_Distance` _returnvalue (`SceneComponent.K2_GetComponentLocation` (`self.Entry/Exit 1`))) (`KismetMathLibrary.Vector_Distance` _returnvalue (`SceneComponent.K2_GetComponentLocation` (`self.Entry/Exit 2`)))))
  (cast `/Game/Entities/Player/BP_Player` OtherActor)
  (`self.OnPlayerEnteredPath` self (`self.IsExitOne`))
  (`KismetSystemLibrary.PrintText` "Hello"))

(fn `UserConstructionScript`
  (locals (lPoint :type "/Game/BehaviourObjects/CameraSysteme/ST_CameraPoints Structure") (NewLocalVar :type "Vector Structure" :default (0.0 0.0 0.0)) (Origine :type "Vector Structure") (UpRight :type "Vector Structure") (UpLeft :type "Vector Structure") (DownRight :type "Vector Structure") (DownLeft :type "Vector Structure"))
  (bind _lpoint (`local.lPoint`))
  (bind _returnvalue (`KismetMathLibrary.MakeRotator` 0.0 (`KismetMathLibrary.BreakVector2D` (break `/Game/BehaviourObjects/CameraSysteme/ST_CameraPoints` _lpoint)) (`.Y` (`KismetMathLibrary.BreakVector2D` (break `/Game/BehaviourObjects/CameraSysteme/ST_CameraPoints` _lpoint)))))
  (bind _returnvalue_2 (* (`KismetMathLibrary.GetUpVector` _returnvalue) (`.CameraFOV_15_13BA261D48E1601009A657A9A67BD0FB` (break `/Game/BehaviourObjects/CameraSysteme/ST_CameraPoints` _lpoint))))
  (bind _returnvalue_3 (* (`KismetMathLibrary.GetRightVector` _returnvalue) (`.CameraFOV_15_13BA261D48E1601009A657A9A67BD0FB` (break `/Game/BehaviourObjects/CameraSysteme/ST_CameraPoints` _lpoint))))
  (bind _returnvalue_4 (* (`KismetMathLibrary.GetForwardVector` _returnvalue) 200.0))
  (bind _returnvalue_5 (+ _returnvalue_4 _returnvalue_3))
  (bind _returnvalue_6 (- _returnvalue_4 _returnvalue_3))
  (`KismetSystemLibrary.FlushPersistentDebugLines`)
  (for (_array_element _array_index) (`self.ArrayPoints`)
    (set `local.lPoint` _array_element)
    (bind _returnvalue_7 (+ (`SplineComponent.GetLocationAtSplinePoint` (`self.Spline`) _array_index "World") (`.CameraOffset_27_0099F0B2440FEB464C0730A823FA62B1` (break `/Game/BehaviourObjects/CameraSysteme/ST_CameraPoints` _lpoint))))
    (set `local.Origine` _returnvalue_7)
    (set `local.UpRight` (+ (+ _returnvalue_5 _returnvalue_2) _returnvalue_7))
    (set `local.UpLeft` (+ (+ _returnvalue_6 _returnvalue_2) _returnvalue_7))
    (set `local.DownRight` (+ (- _returnvalue_5 _returnvalue_2) _returnvalue_7))
    (set `local.DownLeft` (+ (- _returnvalue_6 _returnvalue_2) _returnvalue_7))
    (`KismetSystemLibrary.DrawDebugArrow` (`local.Origine`) (`local.UpLeft`) 1.0 (struct :`B` 1.0 :`A` 1.0) 2000.0 1.0)
    (`KismetSystemLibrary.DrawDebugArrow` (`local.Origine`) (`local.UpRight`) 1.0 (struct :`B` 1.0 :`A` 1.0) 2000.0 1.0)
    (`KismetSystemLibrary.DrawDebugArrow` (`local.Origine`) (`local.DownLeft`) 1.0 (struct :`B` 1.0 :`A` 1.0) 2000.0 1.0)
    (`KismetSystemLibrary.DrawDebugArrow` (`local.Origine`) (`local.DownRight`) 1.0 (struct :`B` 1.0 :`A` 1.0) 2000.0 1.0)
    (`KismetSystemLibrary.DrawDebugArrow` (`local.UpLeft`) (`local.UpRight`) 1.0 (struct :`B` 1.0 :`A` 1.0) 2000.0 1.0)
    (`KismetSystemLibrary.DrawDebugArrow` (`local.UpRight`) (`local.DownRight`) 1.0 (struct :`B` 1.0 :`A` 1.0) 2000.0 1.0)
    (`KismetSystemLibrary.DrawDebugArrow` (`local.DownRight`) (`local.DownLeft`) 1.0 (struct :`B` 1.0 :`A` 1.0) 2000.0 1.0)
    (`KismetSystemLibrary.DrawDebugArrow` (`local.DownLeft`) (`local.UpLeft`) 1.0 (struct :`B` 1.0 :`A` 1.0) 2000.0 1.0)
    (`KismetSystemLibrary.DrawDebugSphere` (`local.Origine`) 25.0 12 (struct :`R` 1.0 :`G` 1.0 :`B` 1.0 :`A` 1.0) 2000.0)))