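; BP_VoiceLine is a trigger-volume actor that plays a voice line with a subtitle when the player enters its box.
; On overlap with a component tagged PlayerCollision, it plays the sound in 2D and sends speaker, text, color and display time to the HUD_Game subtitle system.
; A timer matching the sound's duration clears a playing flag, blocking overlapping playback but allowing the line to replay on later entries.
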(event `self.Box.OnComponentBeginOverlap`
  (params (OverlappedComponent :type "PrimitiveComponent Object Reference") (OtherActor :type "Actor Object Reference") (OtherComp :type "PrimitiveComponent Object Reference") (OtherBodyIndex :type Integer) (bFromSweep :type Boolean) (SweepResult :type "HitResult Structure (by ref)"))
  (bind _soundtoplay (`self.SoundToPlay`))
  (if (`ActorComponent.ComponentHasTag` OtherComp "PlayerCollision")
    (if (not (`self.isSoundPlaying`))
      (set `self.isSoundPlaying` true)
      (`GameplayStatics.PlaySound2D` _soundtoplay 1.0 1.0 0.0 null null)
      (bind _ashud_game (cast `/Game/Core/GameModes/Game/HUD_Game` (`PlayerController.GetHUD` (`GameplayStatics.GetPlayerController` 0))))
      (`/Game/Core/GameModes/Game/HUD_Game.NewLineSubtitle` _ashud_game (`self.Speaker`) (`self.Subtitle Text`) (`self.SpeakerColor`) (`self.DeleteTime`))
      (`KismetSystemLibrary.K2_SetTimerDelegate` (delegate `FinishExecution`) (`SoundBase.Duration` _soundtoplay)))))

(event `FinishExecution`
  (set `self.isSoundPlaying` false))

(fn `UserConstructionScript`)