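; BP_Checkpoint is a trigger actor that saves the player's checkpoint and can play an intro cinematic.
; A player-collision overlap calls SaveCheckpoint, then plays any assigned Level Sequence with Wwise music switching.
; EnablePlayerCamera switches the view to BP_Camera, applies checkpoint camera values and clears the sequence to prevent replays.
; The construction script generates a persistent GUID, copying it and the level to load into CheckpointValue on later runs.
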(event `self.ReceiveBeginPlay`)

(event `self.Trigger.OnComponentBeginOverlap`
  (params (OverlappedComponent :type "PrimitiveComponent Object Reference") (OtherActor :type "Actor Object Reference") (OtherComp :type "PrimitiveComponent Object Reference") (OtherBodyIndex :type Integer) (bFromSweep :type Boolean) (SweepResult :type "HitResult Structure (by ref)"))
  (if (`ActorComponent.ComponentHasTag` OtherComp "PlayerCollision")
    (bind _asbp_player (cast `/Game/Entities/Player/BP_Player` OtherActor))
    (`/Game/Entities/Player/BP_Player.SaveCheckpoint` _asbp_player self (`self.CheckpointValue`))
    (`self.PlayCinematique`)))

(event `PlayCinematique`
  (bind _level_sequence (`self.Level Sequence`)
    (:`then`
      (bind (_outactor _returnvalue) (`LevelSequencePlayer.CreateLevelSequencePlayer` _level_sequence (make `MovieSceneSequencePlaybackSettings` false (struct) (struct :`bAllowRounding` true) 1.0 0.0 false true true true true)))
      (set `self.Out Actor` _outactor)
      (`MovieSceneSequencePlayer.Play` _returnvalue)
      (`AkGameplayStatics.PostEvent` "/Game/WwiseAudio/Events/Default_Work_Unit/MUSIC/Play_MUSIC_menu_loop.Play_MUSIC_menu_loop")
      (`AkGameplayStatics.PostEvent` "/Game/WwiseAudio/Events/Default_Work_Unit/MUSIC/StopSic.StopSic")
      (add `MovieSceneSequencePlayer.OnFinished` _returnvalue (`|CreateDelegate` :!event `EnablePlayerCamera`)))
    (:`else`
      (`self.EnablePlayerCamera`))))

(event `EnablePlayerCamera`
  (bind _returnvalue (`GameplayStatics.GetActorOfClass` "/Game/BehaviourObjects/CameraSysteme/BP_Camera.BP_Camera_C"))
  (`PlayerController.SetViewTargetWithBlend` (`GameplayStatics.GetPlayerController` 0) _returnvalue 0.0 "VTBlend_Linear" 0.0 false)
  (`/Game/BehaviourObjects/CameraSysteme/BP_Camera.SetCameraValueAtCheckPoint` _returnvalue self)
  (set `self.Level Sequence` null)
  (bind _out_actor (`self.Out Actor`)
    (:`then`
      (`self.K2_DestroyActor` _out_actor)
      (`AkGameplayStatics.PostEvent` "/Game/WwiseAudio/Events/Default_Work_Unit/MUSIC/Stop_MUSIC_menu_loop.Stop_MUSIC_menu_loop")
      (`AkGameplayStatics.PostEvent` "/Game/WwiseAudio/Events/Default_Work_Unit/Play_MUSIC_Level.Play_MUSIC_Level"))
    (:`else`)))

(fn `UserConstructionScript`
  (if (not (`KismetStringLibrary.NotEqual_StrStr` (`self.ID`)))
    (set `self.ID` (`KismetGuidLibrary.Conv_GuidToString` (`KismetGuidLibrary.NewGuid`)))
    (else
      (bind _checkpointvalue (`self.CheckpointValue`)
        (:`then`
          (set `/Game/Core/Optimisations/CheckpointSystem/PDA_checkpointValue.CheckpointID` (`self.ID`) _checkpointvalue)
          (set `/Game/Core/Optimisations/CheckpointSystem/PDA_checkpointValue.LevelToLoad` (`self.LevelToLoad`) _checkpointvalue))
        (:`else`)))))