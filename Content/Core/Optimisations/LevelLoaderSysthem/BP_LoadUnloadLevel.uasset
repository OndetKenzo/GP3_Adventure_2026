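; BP_LoadUnloadLevel is a trigger-box actor that starts asynchronous level loading when the player reaches it.
; On overlap with a component tagged PlayerCollision, it can first tell BP_CrowdManager to release agents before loading.
; It then calls LoadLevelsAsync on GM_Base with its configured level list, play-rate modification and a skip-optimised-loading flag.
; Despite its name, it issues no unload call itself.
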(event `self.Box.OnComponentBeginOverlap`
  (params (OverlappedComponent :type "PrimitiveComponent Object Reference") (OtherActor :type "Actor Object Reference") (OtherComp :type "PrimitiveComponent Object Reference") (OtherBodyIndex :type Integer) (bFromSweep :type Boolean) (SweepResult :type "HitResult Structure (by ref)"))
  (if (`ActorComponent.ComponentHasTag` OtherComp "PlayerCollision")
    (`|ExecutionSequence`
      (:`then_0`
        ; Release crowd agent
        (if (`self.ReleaseCrowdAgent`)
          (bind _returnvalue (`GameplayStatics.GetActorOfClass` "/Game/Entities/NPCs/Crowd/BP_CrowdManager.BP_CrowdManager_C"))
          (`/Game/Entities/NPCs/Crowd/BP_CrowdManager.ReleaseAgentBefordLevelLoading` _returnvalue)
          (`KismetSystemLibrary.DelayUntilNextTick`)))
      (:`then_1`
        ; Load level
        (bind _asgm_base (cast `/Game/Core/GameModes/Game/GM_Base` (`GameplayStatics.GetGameMode`)))
        (`/Game/Core/GameModes/Game/GM_Base.LoadLevelsAsync` _asgm_base (`self.LevelToLoad`) true (`self.SkipOptiLoading`))))))

(fn `UserConstructionScript`)