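; Base game mode that loads the saved checkpoint's levels, then places the player at the start position with its cinematic.
; Level streaming is driven by Level Sequence players, created per section in a map and moved to marked frames to load or disable levels.
; It binds to the HUD's respawn event.
; Respawn loading releases crowd agents, reloads the save, and disables then reloads the checkpoint's levels, broadcasting camera and respawn events.
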(event `self.ReceiveBeginPlay`
  ; Load base level
  (`self.InitialiseLevelSequence`)
  (bind _asgi_main (cast `/Game/Core/Saves/GI_Main` (`GameplayStatics.GetGameInstance`)))
  (`/Game/Core/Saves/GI_Main.LoadSave` _asgi_main)
  (bind _checkpointvalue (`/Game/Core/Saves/SGB_Game.CheckpointValue` (`/Game/Core/Saves/GI_Main.SGB_Game` _asgi_main)))
  (`self.OnLoadCamera` _checkpointvalue)
  (`self.LoadLevelsAsync` (`/Game/Core/Optimisations/CheckpointSystem/PDA_checkpointValue.LevelToLoad` _checkpointvalue))
  (`self.SpawnPlayer`)
  (`self.BindEvents`))

(event `SpawnPlayer`
  ; Arbitrare load time
  (`KismetSystemLibrary.Delay` 2.0)
  (bind _asgi_main (cast `/Game/Core/Saves/GI_Main` (`GameplayStatics.GetGameInstance`) :!label _label))
  ; Fix player locaton after spawn
  (bind _checkpoint (`/Game/Core/Saves/GI_Main.GetPlayerStartPosition` _asgi_main))
  (`/Engine/EditorBlueprintResources/StandardMacros.IsValid` _checkpoint
    (:`Is Valid`
      (`/Game/Core/Optimisations/CheckpointSystem/BP_Checkpoint.PlayCinematique` _checkpoint)
      (`self.K2_SetActorTransform` (`GameplayStatics.GetPlayerPawn` 0) (`SceneComponent.K2_GetComponentToWorld` (`/Game/Core/Optimisations/CheckpointSystem/BP_Checkpoint.SM_Gabari` _checkpoint)) false true)
      (`KismetSystemLibrary.Delay` 3.0)
      ; Disable UI loading
      (`self.OnFinishLoadingLevel`))
    (:`Is Not Valid`
      ; Disable UI loading
      (`self.OnFinishLoadingLevel`))))

(event `RespawnPlayer`
  (`KismetSystemLibrary.Delay` 0.2)
  (goto _label))

(event `BindEvents`
  (bind _ashud_game (cast `/Game/Core/GameModes/Game/HUD_Game` (`PlayerController.GetHUD` (`GameplayStatics.GetPlayerController` 0))))
  (add `/Game/Core/GameModes/Game/HUD_Game.OnPlayerRespawn` _ashud_game (`|CreateDelegate` :!event `RespawnPlayer`)))

(event `RespawnLoadLevel`
  (bind _returnvalue (`GameplayStatics.GetActorOfClass` "/Game/Entities/NPCs/Crowd/BP_CrowdManager.BP_CrowdManager_C"))
  (`/Game/Entities/NPCs/Crowd/BP_CrowdManager.ReleaseAgentBefordLevelLoading` _returnvalue)
  (bind _asgi_main (cast `/Game/Core/Saves/GI_Main` (`GameplayStatics.GetGameInstance`)))
  (`/Game/Core/Saves/GI_Main.LoadSave` _asgi_main)
  (bind _checkpointvalue (`/Game/Core/Saves/SGB_Game.CheckpointValue` (`/Game/Core/Saves/GI_Main.SGB_Game` _asgi_main)))
  (`self.OnLoadCamera` _checkpointvalue)
  (bind _leveltoload (`/Game/Core/Optimisations/CheckpointSystem/PDA_checkpointValue.LevelToLoad` _checkpointvalue))
  (`self.DisableLevel` _leveltoload)
  (`KismetSystemLibrary.DelayUntilNextTick`)
  (`self.LoadLevelsAsync` _leveltoload)
  (`self.OnRespawn`))

(fn `DisableLevel`
  (params (Levels :type "Map of /Game/Core/Optimisations/LevelLoaderSysthem/E_LevelName Enum to /Game/Core/Optimisations/LevelLoaderSysthem/E_LoadType Enum (by ref)"))
  (locals (MapValue :type "/Game/Core/Optimisations/LevelLoaderSysthem/E_LoadType Enum") (LevelSequencePlayer :type "LevelSequencePlayer Object Reference") (MapKey :type "/Game/Core/Optimisations/LevelLoaderSysthem/E_LevelName Enum") (DisableKey :type "/Game/Core/Optimisations/LevelLoaderSysthem/E_LoadType Enum" :default "NewEnumerator5"))
  (bind _value (`BlueprintMapLibrary.Map_Find` (`self.LevelSequence`) (`local.MapKey`)))
  (bind (_keypin _valuepin) (`|MapForEach` Levels)
    (:`then`
      (set `local.MapKey` _keypin)
      (set `local.MapValue` _valuepin)
      (`|ExecutionSequence`
        (:`then_0`
          (`/Engine/EditorBlueprintResources/StandardMacros.IsValid` _value
            (:`Is Valid`
              (set `local.LevelSequencePlayer` _value))))
        (:`then_1`
          (`local.LevelSequencePlayer`
            (:`then`
              ; Jump to specify Frame
              (`MovieSceneSequencePlayer.SetPlaybackPosition` (`local.LevelSequencePlayer`) (make `MovieSceneSequencePlaybackParams` (struct :`FrameNumber` (struct)) 0.0 (`|GetEnumeratorNameAsString` (`local.DisableKey`)) (struct) "MarkedFrame" "Jump")))
            (:`else`)))))))

(fn `InitialiseLevelSequence`
  (`|ExecutionSequence`
    (:`then_0`
      (bind (_outactor _returnvalue) (`LevelSequencePlayer.CreateLevelSequencePlayer` "/Game/Core/Optimisations/LevelLoaderSysthem/LevelLoader/LS_FTUE_S1.LS_FTUE_S1"))
      (`self.SetTickableWhenPaused` _outactor true)
      (`BlueprintMapLibrary.Map_Add` (`self.LevelSequence`) "NewEnumerator0" _returnvalue))
    (:`then_1`
      (bind (_outactor_2 _returnvalue_2) (`LevelSequencePlayer.CreateLevelSequencePlayer` "/Game/Core/Optimisations/LevelLoaderSysthem/LevelLoader/LS_FTUE_S2.LS_FTUE_S2"))
      (`self.SetTickableWhenPaused` _outactor_2 true)
      (`BlueprintMapLibrary.Map_Add` (`self.LevelSequence`) "NewEnumerator1" _returnvalue_2))
    (:`then_2`
      (bind (_outactor_3 _returnvalue_3) (`LevelSequencePlayer.CreateLevelSequencePlayer` "/Game/Core/Optimisations/LevelLoaderSysthem/LevelLoader/LS_FTUE_S3.LS_FTUE_S3"))
      (`self.SetTickableWhenPaused` _outactor_3 true)
      (`BlueprintMapLibrary.Map_Add` (`self.LevelSequence`) "NewEnumerator2" _returnvalue_3))
    (:`then_3`
      (bind (_outactor_4 _returnvalue_4) (`LevelSequencePlayer.CreateLevelSequencePlayer` "/Game/Core/Optimisations/LevelLoaderSysthem/LevelLoader/LS_PART1_S1.LS_PART1_S1"))
      (`self.SetTickableWhenPaused` _outactor_4 true)
      (`BlueprintMapLibrary.Map_Add` (`self.LevelSequence`) "NewEnumerator3" _returnvalue_4))
    (:`then_4`
      (bind (_outactor_5 _returnvalue_5) (`LevelSequencePlayer.CreateLevelSequencePlayer` "/Game/Core/Optimisations/LevelLoaderSysthem/LevelLoader/LS_PART1_S2.LS_PART1_S2"))
      (`self.SetTickableWhenPaused` _outactor_5 true)
      (`BlueprintMapLibrary.Map_Add` (`self.LevelSequence`) "NewEnumerator4" _returnvalue_5))
    (:`then_5`
      (bind (_outactor_6 _returnvalue_6) (`LevelSequencePlayer.CreateLevelSequencePlayer` "/Game/Core/Optimisations/LevelLoaderSysthem/LevelLoader/LS_PART1_S3.LS_PART1_S3"))
      (`self.SetTickableWhenPaused` _outactor_6 true)
      (`BlueprintMapLibrary.Map_Add` (`self.LevelSequence`) "NewEnumerator5" _returnvalue_6))
    (:`then_6`
      (bind (_outactor_7 _returnvalue_7) (`LevelSequencePlayer.CreateLevelSequencePlayer` "/Game/Core/Optimisations/LevelLoaderSysthem/LevelLoader/LS_Boss_S1.LS_Boss_S1"))
      (`self.SetTickableWhenPaused` _outactor_7 true)
      (`BlueprintMapLibrary.Map_Add` (`self.LevelSequence`) "NewEnumerator6" _returnvalue_7))
    (:`then_7`
      (bind (_outactor_8 _returnvalue_8) (`LevelSequencePlayer.CreateLevelSequencePlayer` "/Game/Core/Optimisations/LevelLoaderSysthem/LevelLoader/LS_Boss_S2.LS_Boss_S2"))
      (`self.SetTickableWhenPaused` _outactor_8 true)
      (`BlueprintMapLibrary.Map_Add` (`self.LevelSequence`) "NewEnumerator7" _returnvalue_8))
    (:`then_8`
      (bind (_outactor_9 _returnvalue_9) (`LevelSequencePlayer.CreateLevelSequencePlayer` "/Game/Core/Optimisations/LevelLoaderSysthem/LevelLoader/LS_Boss_S3.LS_Boss_S3"))
      (`self.SetTickableWhenPaused` _outactor_9 true)
      (`BlueprintMapLibrary.Map_Add` (`self.LevelSequence`) "NewEnumerator8" _returnvalue_9))))

(fn `LoadLevelsAsync`
  (params (Levels :type "Map of /Game/Core/Optimisations/LevelLoaderSysthem/E_LevelName Enum to /Game/Core/Optimisations/LevelLoaderSysthem/E_LoadType Enum (by ref)") (ModifyPlayRate :type Boolean) (SkipOptiLoad :type Boolean))
  (locals (MapKey :type "/Game/Core/Optimisations/LevelLoaderSysthem/E_LevelName Enum") (MapValue :type "/Game/Core/Optimisations/LevelLoaderSysthem/E_LoadType Enum") (LevelSequencePlayer :type "LevelSequencePlayer Object Reference"))
  (bind _value (`BlueprintMapLibrary.Map_Find` (`self.LevelSequence`) (`local.MapKey`)))
  (bind (_keypin _valuepin) (`|MapForEach` Levels)
    (:`then`
      (set `local.MapKey` _keypin)
      (set `local.MapValue` _valuepin)
      (`|ExecutionSequence`
        (:`then_0`
          (`/Engine/EditorBlueprintResources/StandardMacros.IsValid` _value
            (:`Is Valid`
              (set `local.LevelSequencePlayer` _value)
              (if (`local.ModifyPlayRate`)
                (`MovieSceneSequencePlayer.SetPlayRate` (`local.LevelSequencePlayer`) 2.0)
                (else
                  (`MovieSceneSequencePlayer.SetPlayRate` (`local.LevelSequencePlayer`) 1.0))))
            (:`Is Not Valid`
              ; Debug Error
              (`KismetSystemLibrary.PrintText` (`|FormatText` "Failed to load level {levelName} at position {Position}" (`|GetEnumeratorNameAsString` (`local.MapKey`)) (`|GetEnumeratorNameAsString` (`local.MapValue`)))))))
        (:`then_1`
          (`local.LevelSequencePlayer`
            (:`then`
              (if (`|EnumInequality` (`local.MapValue`) (`self.LevelSecanceFullKey`))
                (`local.SkipOptiLoad`
                  (:`then`
                    ; Jump to specify Frame
                    (`MovieSceneSequencePlayer.SetPlaybackPosition` (`local.LevelSequencePlayer`) (make `MovieSceneSequencePlaybackParams` (struct :`FrameNumber` (struct)) 0.0 (`|GetEnumeratorNameAsString` (`local.MapValue`)) (struct) "MarkedFrame" "Jump")))
                  (:`else`
                    ; Play sequence to optimase full loading
                    (`MovieSceneSequencePlayer.PlayTo` :`self` (`local.LevelSequencePlayer`) :`PlaybackParams` (make `MovieSceneSequencePlaybackParams` (struct :`FrameNumber` (struct)) 0.0 (`|GetEnumeratorNameAsString` (`self.LevelSecanceFullKey`)) (struct) "MarkedFrame") :!label _label)))
                (else
                  (goto _label))))
            (:`else`)))))))

(fn `UserConstructionScript`)