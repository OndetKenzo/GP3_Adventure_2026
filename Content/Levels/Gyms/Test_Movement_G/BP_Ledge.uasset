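; BP_Ledge is a ledge actor in the movement test gym that exposes the dimensions of its Box collider.
; GetColliderDepth doubles the bounds Y extent and scales it by the dot product of a supplied actor forward and the box forward, giving a signed value.
; GetColliderHeight returns the bounds Z extent, which is half the full height.
; The event graph and construction script contain no logic.
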(fn `GetColliderDepth`
  (params (ActorForward :type "Vector Structure"))
  (returns (Depth :type "Float (double-precision)"))
  (return (* (* (`KismetMathLibrary.Dot_VectorVector` ActorForward (`SceneComponent.GetForwardVector` (`self.Box`))) (.y (`.BoxExtent` (`KismetSystemLibrary.GetComponentBounds` (`self.Box`))))) 2.0)))

(fn `GetColliderHeight`
  (returns (BoxHeight :type "Float (double-precision)"))
  (return (.z (`.BoxExtent` (`KismetSystemLibrary.GetComponentBounds` (`self.Box`))))))

(fn `UserConstructionScript`)