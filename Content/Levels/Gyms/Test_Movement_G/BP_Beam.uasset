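; Walkable beam that changes BP_Player's speed state and pulls the player onto its center line when they step onto it.
; Overlapping BeamFloor applies the crossing speed and jump permission, and leaving calls the speed update again with jumping allowed.
; SnapToBeam projects the player onto segment A-B, keeping their height.
; The LerpSnap timeline moves them there with movement disabled, passes the mesh rotation as the line rotator, then restores Walking.
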(event `self.BeamFloor.OnComponentBeginOverlap`
  (params (OverlappedComponent :type "PrimitiveComponent Object Reference") (OtherActor :type "Actor Object Reference") (OtherComp :type "PrimitiveComponent Object Reference") (OtherBodyIndex :type Integer) (bFromSweep :type Boolean) (SweepResult :type "HitResult Structure (by ref)"))
  (bind _as_bp_player (`self.As BP Player`))
  (bind _charactermovement (`Character.CharacterMovement` _as_bp_player))
  ; Slows down player and store current line speed
  (bind _asbp_player (cast `/Game/Entities/Player/BP_Player` OtherActor))
  (bind _output_get (set `self.As BP Player` _asbp_player))
  (if (`ActorComponent.ComponentHasTag` OtherComp "PlayerCollision")
    (`/Game/Entities/Player/BP_Player.Update Speed State` _output_get (`self.is Jump Allowed ?`) true false (`self.BeamCrossSpeed`))
    (bind (_returnvalue_x _returnvalue_y _returnvalue_z) (`self.SnapToBeam`))
    (`CharacterMovementComponent.SetMovementMode` _charactermovement "MOVE_None" 0)
    (bind (_direction _newtrack_0) (`Timeline|LerpSnap` :!via `PlayFromStart`)
      (:`Update`
        (`self.K2_SetActorLocation` (`self.As BP Player`) (`KismetMathLibrary.VLerp` (`self.K2_GetActorLocation` _as_bp_player) (`KismetMathLibrary.MakeVector` _returnvalue_x _returnvalue_y _returnvalue_z) _newtrack_0) false false)
        (set `/Game/Entities/Player/BP_Player.CurrentLineRotator` (`SceneComponent.RelativeRotation` (`self.StaticMesh`)) (`self.As BP Player`)))
      (:`Finished`
        (`CharacterMovementComponent.SetMovementMode` _charactermovement "MOVE_Walking" 0)))))

(event `self.BeamFloor.OnComponentEndOverlap`
  (params (OverlappedComponent :type "PrimitiveComponent Object Reference") (OtherActor :type "Actor Object Reference") (OtherComp :type "PrimitiveComponent Object Reference") (OtherBodyIndex :type Integer))
  ; Revert to normal speed
  (bind _asbp_player (cast `/Game/Entities/Player/BP_Player` OtherActor))
  (`/Game/Entities/Player/BP_Player.Update Speed State` _asbp_player true false false 0.0))

(fn `SnapToBeam`
  (returns (ReturnValue_X :type "Float (double-precision)") (ReturnValue_Y :type "Float (double-precision)") (ReturnValue_Z :type "Float (double-precision)"))
  (locals (NewLocalVar :type "Vector Structure"))
  (bind (_returnvalue_x _returnvalue_y _returnvalue_z) (`KismetMathLibrary.BreakVector` (`SceneComponent.K2_GetComponentLocation` (`Actor.RootComponent` (`self.As BP Player`)))))
  (bind _returnvalue (- (`SceneComponent.K2_GetComponentLocation` (`self.B`)) (`SceneComponent.K2_GetComponentLocation` (`self.A`))))
  (set `self.BeamDirection` (`KismetMathLibrary.Normal` _returnvalue 0.001))
  (set `self.DistanceToPlayer` (- (`SceneComponent.K2_GetComponentLocation` (`Actor.RootComponent` (`self.As BP Player`))) (`SceneComponent.K2_GetComponentLocation` (`self.A`))))
  (set `self.DistanceFromBream` (`KismetMathLibrary.Dot_VectorVector` (`self.BeamDirection`) (`self.DistanceToPlayer`)))
  (bind _output_get (set `self.ClampedDistance` (`KismetMathLibrary.FClamp` (`self.DistanceFromBream`) 0.0 (`KismetMathLibrary.VSize` _returnvalue))))
  (bind (_returnvalue_x_2 _returnvalue_y_2) (`KismetMathLibrary.BreakVector` (+ (`SceneComponent.K2_GetComponentLocation` (`self.A`)) (* _output_get (`self.BeamDirection`)))))
  (return _returnvalue_x_2 _returnvalue_y_2 _returnvalue_z))

(fn `UserConstructionScript`)