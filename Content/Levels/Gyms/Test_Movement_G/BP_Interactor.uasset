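; BP_Interactor is a proximity prompt actor that shows an interaction display widget when the player comes near.
; On BeginPlay it creates a W_InteractDisplay, assigns it to its widget component and passes in the configured texture and FTUE text.
; Overlap events on a sphere toggle the widget's visibility for BP_Player only, guarded by an IsDisplayed flag.
; The construction script scales the widget component by WidgetScale and hides it initially.
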(event `self.ReceiveBeginPlay`
  (bind _returnvalue (`|GenericCreateObject` "/Game/Levels/Gyms/Test_Movement_G/W_InteractDisplay.W_InteractDisplay_C"))
  (bind _output_get (set `self.WidgetClass` _returnvalue))
  (`WidgetComponent.SetWidget` (`self.Widget`) _output_get)
  (set `/Game/Levels/Gyms/Test_Movement_G/W_InteractDisplay.ImageTexture` (`self.Texture`) (`self.WidgetClass`))
  (set `/Game/Levels/Gyms/Test_Movement_G/W_InteractDisplay.TextFTUe` (`self.TextFTUE`) (`self.WidgetClass`)))

(event `self.Sphere.OnComponentBeginOverlap`
  (params (OverlappedComponent :type "PrimitiveComponent Object Reference") (OtherActor :type "Actor Object Reference") (OtherComp :type "PrimitiveComponent Object Reference") (OtherBodyIndex :type Integer) (bFromSweep :type Boolean) (SweepResult :type "HitResult Structure (by ref)"))
  (cast `/Game/Entities/Player/BP_Player` OtherActor)
  (if (not (`self.isDisplayed`))
    (set `self.isDisplayed` true)
    (`SceneComponent.SetVisibility` (`self.Widget`) true true)))

(event `self.Sphere.OnComponentEndOverlap`
  (params (OverlappedComponent :type "PrimitiveComponent Object Reference") (OtherActor :type "Actor Object Reference") (OtherComp :type "PrimitiveComponent Object Reference") (OtherBodyIndex :type Integer))
  (cast `/Game/Entities/Player/BP_Player` OtherActor)
  (if (`self.isDisplayed`)
    (set `self.isDisplayed` false)
    (`SceneComponent.SetVisibility` (`self.Widget`) false true)))

(fn `UserConstructionScript`
  (bind _widget (`self.Widget`))
  (`SceneComponent.SetWorldScale3D` _widget (`KismetMathLibrary.Conv_DoubleToVector` (`self.WidgetScale`)))
  (`SceneComponent.SetVisibility` _widget false false))